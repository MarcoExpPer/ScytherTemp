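; Music controller for the final combat zone, driving FMOD boss music from the events of a CombatZone.
; Combat start restores the GameMusic bus volume, plays Boss_Music as a 2D event and keeps the instance.
; Each finished round maps the current round number to a "Battlephase" parameter value through ChangeGameMusic, with several rounds sharing a phase.
; Combat end sets that parameter to its final phase.
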(event CombatStartsEvent(CombatZone)
  (Class|FMODBlueprintStatics|BusSetVolume "/Game/FMOD/Buses/GameMusic.GameMusic" 1.0)
  (bind _returnvalue (Class|FMODBlueprintStatics|PlayEvent2D "/Game/FMOD/Events/Music/Game/Boss_Music.Boss_Music"))
  (Variables|Default|SetGameMusicInstance _returnvalue))

(event CombatEndsEvent(CombatZone)
  (CallFunction|ChangeGameMusic 3.0))

(event CombatRoundFinished(CombatZone)
  ;[1 1 1] Para añadir el sonido del gusano entre rondas de la combat zone
  (switch int (Variables|/Script/Scyther.CombatZone|GetcurrentRound (Variables|Default|GetCombatZone))
    (:0
      (CallFunction|ChangeGameMusic 0.0 :!label _label))
    (:1
      (goto _label))
    (:2
      (CallFunction|ChangeGameMusic 1.0 :!label _label_2))
    (:3
      (goto _label_2))
    (:4
      (CallFunction|ChangeGameMusic 2.0))
    (:5
      (goto _label_2))))

(event Custom|ChangeGameMusic
  (params (TypeOfMusic :type Float%20%28single-precision%29))
  (Class|FMODBlueprintStatics|EventInstanceSetParameter (Variables|Default|GetGameMusicInstance) "Battlephase" TypeOfMusic))

(fn ConstructionScript)