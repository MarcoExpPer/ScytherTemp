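; Combat zone music controller that reacts to the start, end and round-finished events of a CombatZone.
; On start and end it switches between combat and out-of-combat tracks through a cached BP_GameInstance, raising the FMOD GameMusic bus volume during combat and restoring it afterwards.
; When a round finishes, it waits a configurable delay and plays a 2D FMOD event, noted as the worm sound between rounds.
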(event CombatStartsEvent(CombatZone)
  (Utilities|IsValid (Variables|Default|GetBP_GameInstance)
    (:Is%20Valid
      _)
    (:Is%20Not%20Valid
      (bind _asbp_game_instance (Utilities|Casting|CastToBP_GameInstance (Game|GetGameInstance)))
      (bind _output_get (Variables|Default|SetBP_GameInstance _asbp_game_instance))))
  (Default|ChangeGameMusic _output_get (Variables|Audio|GetCombatMusic))
  (Class|FMODBlueprintStatics|BusSetVolume "/Game/FMOD/Buses/GameMusic.GameMusic" 1.25))

(event CombatEndsEvent(CombatZone)
  (Utilities|IsValid (Variables|Default|GetBP_GameInstance)
    (:Is%20Valid
      _)
    (:Is%20Not%20Valid
      (bind _asbp_game_instance (Utilities|Casting|CastToBP_GameInstance (Game|GetGameInstance)))
      (bind _output_get (Variables|Default|SetBP_GameInstance _asbp_game_instance))))
  (Default|ChangeGameMusic _output_get (Variables|Audio|GetOurOfCombatMusic))
  (Class|FMODBlueprintStatics|BusSetVolume "/Game/FMOD/Buses/GameMusic.GameMusic" 1.0))

(event CombatRoundFinished(CombatZone)
  ;[1 1 1] Para añadir el sonido del gusano entre rondas de la combat zone
  (Utilities|FlowControl|Delay (Variables|Audio|GetDurationToSpawnSound))
  (Class|FMODBlueprintStatics|PlayEvent2D (Variables|Audio|GetEvent)))

(fn ConstructionScript)