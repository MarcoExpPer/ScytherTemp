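; Swamp ambience trigger actor that switches an FMOD ambience parameter as the player enters and leaves a box volume.
; Overlaps from components tagged PlayerBody set TipoAmbiente on the audio component to one on entry and zero on exit.
; When the SwampValue flag is set, Tick prints the parameter's current final value to the screen.
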(event OnComponentBeginOverlap(Box)
  (params (OverlappedComponent :type Primitive%20Component%20Object%20Reference) (OtherActor :type Actor%20Object%20Reference) (OtherComp :type Primitive%20Component%20Object%20Reference) (OtherBodyIndex :type Integer) (bFromSweep :type Boolean) (SweepResult :type Hit%20Result%20Structure%20%28by%20ref%29))
  (if (Components|ComponentHasTag OtherComp "PlayerBody")
    (Class|FMODAudioComponent|SetParameter (Variables|Default|GetAudioComponent) "TipoAmbiente" 1.0)))

(event OnComponentEndOverlap(Box)
  (params (OverlappedComponent :type Primitive%20Component%20Object%20Reference) (OtherActor :type Actor%20Object%20Reference) (OtherComp :type Primitive%20Component%20Object%20Reference) (OtherBodyIndex :type Integer))
  (if (Components|ComponentHasTag OtherComp "PlayerBody")
    (Class|FMODAudioComponent|SetParameter (Variables|Default|GetAudioComponent) "TipoAmbiente" 0.0)))

(event EventTick
  (params (DeltaSeconds :type Float%20%28single-precision%29))
  (if (Variables|Sound|GetSwampValue)
    (bind _finalvalue (Class|FMODAudioComponent|GetParameterValue (Variables|Default|GetAudioComponent) "TipoAmbiente"))
    (Development|PrintString (Utilities|String|ToString(Float) _finalvalue) true true "(R=0.009540,G=1.000000,B=0.162746,A=1.000000)" 0.0)))

(fn ConstructionScript)