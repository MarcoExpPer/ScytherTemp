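; In-game HUD Blueprint that owns the gameplay UI, pause menu and death screen widgets.
; After a short BeginPlay delay, it creates the widgets and binds to the game mode's respawn manager, showing the death screen on death and resetting UI on respawn.
; Pause toggling uses a FlipFlop, gated by menu-state flags, to switch game pause, cursor, input mode and audio bus pausing.
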(event Custom|ResetUI
  (params (location :type Vector))
  ;[1 1 1] Bind player respawn/dead events
  ;;[1 1 1] When player respawn
  (Default|Reset (Variables|Default|GetInGame_WG))
  (Default|DeActivate (Variables|Default|GetYouDead_WG)))

(event Custom|TogglePauseMenu
  (bind _returnvalue (Game|GetPlayerController 0))
  (bind _pause_wg (Variables|Default|GetPause_WG))
  ;[1 1 1] Pause input only works from pause menu
  (if (and (Variables|Default|GetisOnMainpauseMenu) (Variables|Default|GetisNOTgoingToCredits))
    (Utilities|FlowControl|FlipFlop
      (:A
        ;[1 1 1] Show pause menu and stop the game
        (UserInterface|Viewport|AddtoViewport (Variables|Default|GetPause_WG) 0)
        (Game|SetGamePaused true)
        (Variables|/Script/Engine.PlayerController|SetbShowMouseCursor (Game|GetPlayerController 0) true)
        (Widget|SetKeyboardFocus (Variables|Default|GetPause_WG))
        (CallFunction|PauseAudio true)
        (Input|SetInputModeUIOnly _returnvalue _pause_wg "LockOnCapture")
        (Input|SetInputModeGameandUI _returnvalue _pause_wg "LockOnCapture" false))
      (:B
        ;[1 1 1] Remove pause menu and play the game again
        (Widget|RemovefromParent (Variables|Default|GetPause_WG))
        (Variables|/Script/Engine.PlayerController|SetbShowMouseCursor (Game|GetPlayerController 0) false)
        (CallFunction|PauseAudio false)
        ;;[1 1 1] To remove buttons from pause menu list, when exiting from player pause btn
        (Default|CleanBtns (Variables|Default|GetPause_WG))
        (Variables|Default|SetisOnMainpauseMenu true)
        (Utilities|FlowControl|Delay 0.05)
        (Game|SetGamePaused false)
        (Input|SetInputModeGameOnly (Game|GetPlayerController 0))))))

(event Custom|PlayerDead
  (bind _youdead_wg (Variables|Default|GetYouDead_WG))
  ;[1 1 1] Bind player respawn/dead events
  ;;[1 1 1] When player dies
  (UserInterface|Viewport|AddtoViewport _youdead_wg 0)
  (Default|Activate _youdead_wg))

(event Custom|BindEvents
  ;[1 1 1] Bind player respawn/dead events
  (bind _asbp_game_mode (Utilities|Casting|CastToBP_GameMode (Game|GetGameMode)))
  (EventDispatchers|BindEventtoPlayerRespawnEvent (Variables|/Script/Scyther.ScytherGameModeBase|GetrespawnMan _asbp_game_mode) (delegate Custom|ResetUI))
  (EventDispatchers|BindEventtoPlayerDeadEvent (Variables|/Script/Scyther.ScytherGameModeBase|GetrespawnMan _asbp_game_mode) (delegate Custom|PlayerDead)))

(event EventBeginPlay
  ;[1 1 1] Delay necesario para pillar bien los eventos del respawn manager
  (Utilities|FlowControl|Delay 0.2)
  (bind _returnvalue (UserInterface|CreateWidget "/Game/HUD/BluePrints/InGameHud/WG_InGameUI.WG_InGameUI_C"))
  (bind _output_get (Variables|Default|SetInGame_WG _returnvalue))
  (UserInterface|Viewport|AddtoViewport _output_get 0)
  (bind _returnvalue_2 (UserInterface|CreateWidget "/Game/HUD/BluePrints/InGameHud/WG_PauseMenu.WG_PauseMenu_C"))
  (Variables|Default|SetPause_WG _returnvalue_2)
  (bind _returnvalue_3 (UserInterface|CreateWidget "/Game/HUD/BluePrints/YouDeadHud/WG_YouDead.WG_YouDead_C"))
  (Variables|Default|SetYouDead_WG _returnvalue_3)
  (CallFunction|BindEvents)
  (bind _asbp_scyther_player_controller (Utilities|Casting|CastToBP_ScytherPlayerController (Game|GetPlayerController 0)))
  (Variables|Default|SetplayerController _asbp_scyther_player_controller))

(event EventTogglePauseHUD
  (CallFunction|TogglePauseMenu))

(fn ConstructionScript)

(fn PauseAudio
  (params (pauseMusic? :type Boolean))
  (Class|FMODBlueprintStatics|BusSetPaused "/Game/FMOD/Buses/Ambient.Ambient" pauseMusic?)
  (Class|FMODBlueprintStatics|BusSetPaused "/Game/FMOD/Buses/GameMusic.GameMusic" pauseMusic?)
  (Class|FMODBlueprintStatics|BusSetPaused "/Game/FMOD/Buses/GameSFX.GameSFX" pauseMusic?)
  (Class|FMODBlueprintStatics|BusSetPaused "/Game/FMOD/Buses/Reverb.Reverb" pauseMusic?))