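; Trigger volume that sends the player into the credits when an overlapping component tagged PlayerBody enters its box.
; Caches the BP_InGameHud reference on BeginPlay and clears its IsNOTgoingToCredits flag on overlap.
; The overlap also removes all widgets and shows WG_CreditsWithFadeOut with keyboard focus.
; After a short delay it switches to UI-only input and disables input on the player pawn.
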(event OnComponentBeginOverlap(Box)
  (params (OverlappedComponent :type Primitive%20Component%20Object%20Reference) (OtherActor :type Actor%20Object%20Reference) (OtherComp :type Primitive%20Component%20Object%20Reference) (OtherBodyIndex :type Integer) (bFromSweep :type Boolean) (SweepResult :type Hit%20Result%20Structure%20%28by%20ref%29))
  (bind _returnvalue (Game|GetPlayerController 0))
  (if (Components|ComponentHasTag OtherComp "PlayerBody")
    (Variables|/Game/HUD/BluePrints/InGameHud/BP_InGameHud.BP_InGameHud_C|SetisNOTgoingToCredits (Variables|Default|GetAs%20BP%20In%20Game%20Hud) false)
    (Viewport|RemoveAllWidgets)
    (bind _returnvalue_2 (UserInterface|CreateWidget "/Game/HUD/BluePrints/Credits/WG_CreditsWithFadeOut.WG_CreditsWithFadeOut_C" (Game|GetPlayerController 0)))
    (UserInterface|Viewport|AddtoViewport _returnvalue_2 0)
    (Widget|SetKeyboardFocus _returnvalue_2)
    (Utilities|FlowControl|Delay 1.0)
    (Input|SetInputModeUIOnly _returnvalue 0 "LockOnCapture")
    (Input|DisableInput (Game|Player|GetPlayerPawn 0) _returnvalue)))

(event EventBeginPlay
  (bind _asbp_in_game_hud (Utilities|Casting|CastToBP_InGameHud (HUD|GetHUD (Game|GetPlayerController 0))))
  (Variables|Default|SetAs%20BP%20In%20Game%20Hud _asbp_in_game_hud))

(fn ConstructionScript)