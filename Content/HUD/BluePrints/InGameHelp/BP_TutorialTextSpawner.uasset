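; BP_TutorialTextSpawner is a placed actor that shows a tutorial text widget while the player is inside its ShowBox.
; PlayerBody-tagged overlaps show or hide the WG_TutorialText, with a delayed BeginPlay check catching a player already inside.
; It binds to BP_GameMode's gamepad updates to switch the prompt between keyboard and gamepad, hiding it on gamepad unless ShowWhileUsingKeypad is set.
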(event OnComponentBeginOverlap(ShowBox)
  (params (OverlappedComponent :type Primitive%20Component%20Object%20Reference) (OtherActor :type Actor%20Object%20Reference) (OtherComp :type Primitive%20Component%20Object%20Reference) (OtherBodyIndex :type Integer) (bFromSweep :type Boolean) (SweepResult :type Hit%20Result%20Structure%20%28by%20ref%29))
  (bind _as_wg_tutorial_text (Variables|Default|GetAs%20WG%20Tutorial%20Text))
  (if (Components|ComponentHasTag OtherComp "PlayerBody")
    (if (Utilities|IsValid _as_wg_tutorial_text)
      (Default|Show _as_wg_tutorial_text)
      ;[1 1 1] Check if must be active on begin play
      (Utilities|Array|ForEachLoopwithBreak (Class|PrimitiveComponent|GetOverlappingComponents (Variables|Default|GetShowBox))) ; enters at Break
    )))

(event OnComponentEndOverlap(ShowBox)
  (params (OverlappedComponent :type Primitive%20Component%20Object%20Reference) (OtherActor :type Actor%20Object%20Reference) (OtherComp :type Primitive%20Component%20Object%20Reference) (OtherBodyIndex :type Integer))
  (if (Components|ComponentHasTag OtherComp "PlayerBody")
    (Default|Hide (Variables|Default|GetAs%20WG%20Tutorial%20Text))))

(event Custom|OnUsingGamepadChange
  (params (isUsingGamepad :type Boolean))
  ;[1 1 1] Bind to gamepad update
  (CallFunction|UpdateWidget isUsingGamepad))

(event EventBeginPlay
  (Utilities|FlowControl|Sequence
    (:then_0
      ;[1 1 1] Cast to tutorialText
      (bind _aswg_tutorial_text (Utilities|Casting|CastToWG_TutorialText (UserInterface|GetWidget (Variables|Default|GetWidget))))
      (Variables|Default|SetAs%20WG%20Tutorial%20Text _aswg_tutorial_text))
    (:then_1
      ;[1 1 1] Bind to gamepad update
      (bind _asbp_game_mode (Utilities|Casting|CastToBP_GameMode (Game|GetGameMode)))
      (EventDispatchers|BindEventtoIsUsingGamepadUpdated _asbp_game_mode (delegate Custom|OnUsingGamepadChange))
      (CallFunction|UpdateWidget (Variables|/Game/Blueprints/Managers/BP_GameMode.BP_GameMode_C|GetisUsingGamepad? _asbp_game_mode)))
    (:then_2
      (Utilities|FlowControl|Delay 0.5)
      ;[1 1 1] Check if must be active on begin play
      (bind _array_element (Utilities|Array|ForEachLoopwithBreak (Class|PrimitiveComponent|GetOverlappingComponents (Variables|Default|GetShowBox)))
        (:LoopBody
          (if (and (Components|ComponentHasTag _array_element "PlayerBody") (Utilities|IsValid (Variables|Default|GetAs%20WG%20Tutorial%20Text)))
            (Default|Show (Variables|Default|GetAs%20WG%20Tutorial%20Text))))))))

(fn ConstructionScript)

(fn UpdateWidget
  (params (isUsingGamepad :type Boolean))
  (if isUsingGamepad
    (if (Variables|Default|GetshowWhileUsingKeypad?)
      (Default|UpdateWidget (Variables|Default|GetAs%20WG%20Tutorial%20Text) (Variables|Default|Gettext) (Variables|Default|GetinputType) false)
      (else
        (Rendering|SetVisibility (Variables|Default|GetWidget) false true)))
    (else
      (Rendering|SetVisibility (Variables|Default|GetWidget) true true)
      (Default|UpdateWidget (Variables|Default|GetAs%20WG%20Tutorial%20Text) (Variables|Default|Gettext) (Variables|Default|GetinputType) true))))