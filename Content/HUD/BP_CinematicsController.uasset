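; BP_CinematicsController is a controller for cinematics that lets the player stop the teaser or credits video.
; Pause, Jump and Enter presses share one path that finds a top-level WG_Teaser widget, falling back to WG_Credits, and calls StopVideo on it.
; Any key press also tracks gamepad versus non-gamepad input and fires GamepadStateChanged when that state changes.
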(event EventBeginPlay)

(event EventTick
  (params (DeltaSeconds :type Float%20%28single-precision%29)))

(event Input|ActionEvents|InputActionPause
  (params (Key :type Key%20Structure :default "None"))
  (:Pressed
    (bind _foundwidgets (Widget|GetAllWidgetsOfClass "/Game/HUD/BluePrints/Teaser/WG_Teaser.WG_Teaser_C" true))
    (if (!= (Utilities|Array|Length _foundwidgets) 0)
      (Default|StopVideo (Utilities|Array|Get(acopy) _foundwidgets))
      (else
        (bind _foundwidgets_2 (Widget|GetAllWidgetsOfClass "/Game/HUD/BluePrints/Credits/WG_Credits.WG_Credits_C" true))
        (if (!= (Utilities|Array|Length _foundwidgets_2) 0)
          (Default|StopVideo (Utilities|Array|Get(acopy) _foundwidgets_2)))))))

(event Input|ActionEvents|InputActionJump
  (params (Key :type Key%20Structure :default "None"))
  (:Pressed
    (bind _foundwidgets (Widget|GetAllWidgetsOfClass "/Game/HUD/BluePrints/Teaser/WG_Teaser.WG_Teaser_C" true))
    (if (!= (Utilities|Array|Length _foundwidgets) 0)
      (Default|StopVideo (Utilities|Array|Get(acopy) _foundwidgets))
      (else
        (bind _foundwidgets_2 (Widget|GetAllWidgetsOfClass "/Game/HUD/BluePrints/Credits/WG_Credits.WG_Credits_C" true))
        (if (!= (Utilities|Array|Length _foundwidgets_2) 0)
          (Default|StopVideo (Utilities|Array|Get(acopy) _foundwidgets_2)))))))

(event Input|KeyboardEvents|Enter
  (params (Key :type Key%20Structure :default "None"))
  (:Pressed
    (bind _foundwidgets (Widget|GetAllWidgetsOfClass "/Game/HUD/BluePrints/Teaser/WG_Teaser.WG_Teaser_C" true))
    (if (!= (Utilities|Array|Length _foundwidgets) 0)
      (Default|StopVideo (Utilities|Array|Get(acopy) _foundwidgets))
      (else
        (bind _foundwidgets_2 (Widget|GetAllWidgetsOfClass "/Game/HUD/BluePrints/Credits/WG_Credits.WG_Credits_C" true))
        (if (!= (Utilities|Array|Length _foundwidgets_2) 0)
          (Default|StopVideo (Utilities|Array|Get(acopy) _foundwidgets_2)))))))

(event Input|KeyboardEvents|AnyKey
  (params (Key :type Key%20Structure :default "None"))
  (bind _returnvalue (Class|KismetInputLibrary|KeyIsGamepadKey Key))
  (:Pressed
    (if (Math|Boolean|NotEqual(Boolean) _returnvalue (Variables|Default|GetisUsingGamepad?))
      (bind _output_get (Variables|Default|SetisUsingGamepad? _returnvalue))
      (Default|CallGamepadStateChanged _output_get))))

(fn ConstructionScript)