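; BP_BreakableFloor is a floor piece that breaks shortly after the player steps on it.
; An overlap of TriggerBreakObject by a component tagged PlayerBody rotates the actor locally as a cue and sets IsBreaking so the sequence starts only once.
; After the TimeToBreak delay, the actor sends DEADZONE damage to its Health, leaving the actual breaking to that damage handling.
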(event OnComponentBeginOverlap(TriggerBreakObject)
  (params (OverlappedComponent :type Primitive%20Component%20Object%20Reference) (OtherActor :type Actor%20Object%20Reference) (OtherComp :type Primitive%20Component%20Object%20Reference) (OtherBodyIndex :type Integer) (bFromSweep :type Boolean) (SweepResult :type Hit%20Result%20Structure%20%28by%20ref%29))
  (if (Components|ComponentHasTag OtherComp "PlayerBody")
    (if (not (Variables|Default|GetisBreaking))
      (Transformation|AddActorLocalRotation (Variables|Default|Getrotation) false false)
      (Variables|Default|SetisBreaking true)
      (Utilities|FlowControl|Delay (Variables|Default|GettimeToBreak))
      (Class|HealthComponent|ReceiveDamage (Variables|Default|GetHealth) 1e+01 "DEADZONE" true))))

(fn ConstructionScript)