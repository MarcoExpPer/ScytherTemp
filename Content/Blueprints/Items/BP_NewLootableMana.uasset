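; Lootable mana pickup in light or dark variants, with material and Niagara effect chosen by IsLightMana.
; When looted with DoUIAnimation set, a timeline flies it toward the HUD mana bar by deprojecting the widget's approximate screen position into world space.
; On arrival it hides, credits mana through the player's SkillComponent, and destroys itself unless it comes from the world.
; Respawn stops the timeline before running parent logic.
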(event Custom|IsLightManaChangedEvent_Event_0
  (if (Variables|Default|GetisLightMana)
    (CallFunction|ChangeLightNiagara)
    (else
      (CallFunction|ChangeDarkNiagara))))

(event Custom|startUIAnimation
  (bind _returnvalue (Game|GetPlayerController 0))
  (bind _realhud (Variables|Default|GetRealHud))
  (bind _ingame_wg (Variables|/Game/HUD/BluePrints/InGameHud/BP_InGameHud.BP_InGameHud_C|GetInGame_WG _realhud))
  (bind _mpbar_1_background (Variables|/Game/HUD/BluePrints/InGameHud/WG_InGameUI.WG_InGameUI_C|GetMPBar_1_Background _ingame_wg))
  (bind _returnvalue_2 (Class|WidgetLayoutLibrary|SlotasCanvasSlot _mpbar_1_background))
  (bind _returnvalue_3 (Class|Widget|GetCachedGeometry _mpbar_1_background))
  (bind _returnvalue_4 (Class|CanvasPanelSlot|GetPosition _returnvalue_2))
  (bind _returnvalue_5 (Class|CanvasPanelSlot|GetSize _returnvalue_2))
  (bind _returnvalue_6 (/ (.x _returnvalue_5) 2.0))
  (bind _returnvalue_7 (* 3 (.y _returnvalue_5)))
  (bind _viewportposition (Class|SlateBlueprintLibrary|LocaltoViewport _returnvalue_3 _returnvalue_4))
  (bind _returnvalue_8 (- (.y _viewportposition) _returnvalue_7))
  (bind _returnvalue_9 (- (.x _viewportposition) _returnvalue_6))
  (bind (_worldlocation _worlddirection) (Class|PlayerController|DeprojectScreenPositiontoWorld _returnvalue _returnvalue_9 _returnvalue_8))
  (if (Variables|Default|GetdoUIAnimation)
    (Variables|Default|SetstartLocation (Transformation|GetActorLocation))
    (Utilities|FlowControl|Sequence
      (:then_0
        (bind _newtrack_0 (Timeline|Timeline_0 PlayFromStart)
          (:Update
            (Transformation|SetActorLocation (Math|Vector|Lerp(Vector) (Variables|Default|GetstartLocation) (+ _worldlocation (* _worlddirection 3.5e+03)) _newtrack_0) false false))
          (:Finished
            (Rendering|SetActorHiddenInGame true)
            (bind _asscyther_player_pawn (Utilities|Casting|CastToScytherPlayerPawn (Game|Player|GetPlayerPawn 0)))
            (Class|SkillComponent|UpdateMana (Variables|/Script/Scyther.ScytherPlayerPawn|GetskillComponent _asscyther_player_pawn) (Variables|Default|GetisLightMana) (Variables|Default|GetmanaAmount))
            (if (not (Variables|Default|GetisFromWorld))
              (Actor|DestroyActor))))))))

(event EventBeginPlay
  (bind _asbp_in_game_hud (Utilities|Casting|CastToBP_InGameHud (HUD|GetHUD (Game|GetPlayerController 0))))
  (Variables|Default|SetRealHud _asbp_in_game_hud)
  (EventDispatchers|BindEventtoLootedEvent (delegate Custom|startUIAnimation))
  (EventDispatchers|AssignIsLightManaChangedEvent (delegate Custom|IsLightManaChangedEvent_Event_0))
  (if (Variables|Default|GetisLightMana)
    (CallFunction|ChangeLightNiagara)
    (else
      (CallFunction|ChangeDarkNiagara))))

(event EventRespawn
  (bind _returnvalue (Game|GetPlayerController 0))
  (bind _realhud (Variables|Default|GetRealHud))
  (bind _ingame_wg (Variables|/Game/HUD/BluePrints/InGameHud/BP_InGameHud.BP_InGameHud_C|GetInGame_WG _realhud))
  (bind _mpbar_1_background (Variables|/Game/HUD/BluePrints/InGameHud/WG_InGameUI.WG_InGameUI_C|GetMPBar_1_Background _ingame_wg))
  (bind _returnvalue_2 (Class|WidgetLayoutLibrary|SlotasCanvasSlot _mpbar_1_background))
  (bind _returnvalue_3 (Class|Widget|GetCachedGeometry _mpbar_1_background))
  (bind _returnvalue_4 (Class|CanvasPanelSlot|GetPosition _returnvalue_2))
  (bind _returnvalue_5 (Class|CanvasPanelSlot|GetSize _returnvalue_2))
  (bind _returnvalue_6 (/ (.x _returnvalue_5) 2.0))
  (bind _returnvalue_7 (* 3 (.y _returnvalue_5)))
  (bind _viewportposition (Class|SlateBlueprintLibrary|LocaltoViewport _returnvalue_3 _returnvalue_4))
  (bind _returnvalue_8 (- (.y _viewportposition) _returnvalue_7))
  (bind _returnvalue_9 (- (.x _viewportposition) _returnvalue_6))
  (bind (_worldlocation _worlddirection) (Class|PlayerController|DeprojectScreenPositiontoWorld _returnvalue _returnvalue_9 _returnvalue_8))
  (Utilities|FlowControl|Sequence
    (:then_0
      (bind _newtrack_0 (Timeline|Timeline_0 Stop)
        (:Update
          (Transformation|SetActorLocation (Math|Vector|Lerp(Vector) (Variables|Default|GetstartLocation) (+ _worldlocation (* _worlddirection 3.5e+03)) _newtrack_0) false false))
        (:Finished
          (Rendering|SetActorHiddenInGame true)
          (bind _asscyther_player_pawn (Utilities|Casting|CastToScytherPlayerPawn (Game|Player|GetPlayerPawn 0)))
          (Class|SkillComponent|UpdateMana (Variables|/Script/Scyther.ScytherPlayerPawn|GetskillComponent _asscyther_player_pawn) (Variables|Default|GetisLightMana) (Variables|Default|GetmanaAmount))
          (if (not (Variables|Default|GetisFromWorld))
            (Actor|DestroyActor)))))
    (:then_1
      (|CallParentFunction))))

(fn ConstructionScript
  (Rendering|Material|SetMaterial (Variables|Character|GetMesh) 0 (select (Variables|Default|GetisLightMana) "/Game/Arte/Escena1/Enemies/Generic/Materials/M_Light.M_Light" "/Game/Arte/Escena1/Enemies/Generic/Materials/M_Dark.M_Dark"))
  (if (Variables|Default|GetisLightMana)
    (CallFunction|ChangeLightNiagara)
    (else
      (CallFunction|ChangeDarkNiagara))))

(fn ChangeLightNiagara
  (Components|Activation|Activate (Variables|Default|GetNiagara_Light) true)
  (Components|Activation|Deactivate (Variables|Default|GetNiagara_dark)))

(fn ChangeDarkNiagara
  (Components|Activation|Activate (Variables|Default|GetNiagara_dark) true)
  (Components|Activation|Deactivate (Variables|Default|GetNiagara_Light)))