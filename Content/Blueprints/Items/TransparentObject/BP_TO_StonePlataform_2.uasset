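; A transparent-object stone platform that fades out while the player's body is inside its trigger box and fades back in afterwards.
; Overlap events on HideMeshWhenInsideThisBox check for the PlayerBody component tag and toggle a disappearing flag.
; Tick reads the flag and steps opacity at a set rate toward a minimum or full opacity, writing it to the Destructible component's material Opacity parameter.
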(event OnComponentBeginOverlap(HideMeshWhenInsideThisBox)
  (params (OverlappedComponent :type Primitive%20Component%20Object%20Reference) (OtherActor :type Actor%20Object%20Reference) (OtherComp :type Primitive%20Component%20Object%20Reference) (OtherBodyIndex :type Integer) (bFromSweep :type Boolean) (SweepResult :type Hit%20Result%20Structure%20%28by%20ref%29))
  (if (Components|ComponentHasTag OtherComp "PlayerBody")
    (Variables|Default|SetIsDissapearing? true)))

(event OnComponentEndOverlap(HideMeshWhenInsideThisBox)
  (params (OverlappedComponent :type Primitive%20Component%20Object%20Reference) (OtherActor :type Actor%20Object%20Reference) (OtherComp :type Primitive%20Component%20Object%20Reference) (OtherBodyIndex :type Integer))
  (if (Components|ComponentHasTag OtherComp "PlayerBody")
    (Variables|Default|SetIsDissapearing? false)))

(event EventBeginPlay
  (|CallParentFunction)
  (Variables|Default|SetcurrentOpacity 1.0))

(event Collision|EventActorBeginOverlap
  (params (OtherActor :type Actor%20Object%20Reference)))

(event EventTick
  (params (DeltaSeconds :type Float%20%28single-precision%29))
  (|CallParentFunction DeltaSeconds)
  (if (Variables|Default|GetIsDissapearing?)
    (if (and (<= (Variables|Default|GetcurrentOpacity) 1.0) (!= (Variables|Default|GetcurrentOpacity) (Variables|Default|GetminimumOpactiy)))
      (CallFunction|ReduceOpacity DeltaSeconds))
    (elif (and (>= (Variables|Default|GetcurrentOpacity) 0.0) (!= (Variables|Default|GetcurrentOpacity) 1.0))
      (CallFunction|IncreaseOpacity DeltaSeconds))))

(fn ConstructionScript
  (|CallParentFunction))

(fn ReduceOpacity
  (params (DeltaTime :type Float%20%28single-precision%29))
  (bind _output_get (Variables|Default|SetcurrentOpacity (Math|Float|Max(Float) (- (Variables|Default|GetcurrentOpacity) (* DeltaTime (Variables|Default|GetopacityStep))) (Variables|Default|GetminimumOpactiy))))
  (Rendering|Material|SetScalarParameterValueonMaterials (Variables|Default|GetDestructible) "Opacity" _output_get))

(fn IncreaseOpacity
  (params (DeltaTime :type Float%20%28single-precision%29))
  (bind _output_get (Variables|Default|SetcurrentOpacity (Math|Float|Min(Float) (+ (Variables|Default|GetcurrentOpacity) (* DeltaTime (Variables|Default|GetopacityStep))) 1.0)))
  (Rendering|Material|SetScalarParameterValueonMaterials (Variables|Default|GetDestructible) "Opacity" _output_get))