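; BP_ShadowArea is a box volume that marks a dark area, notifying actors as they enter or leave shadow.
; Overlap begin and end send EnterDarkArea and EnterLightArea messages to actors implementing CanEnterDarkLightAreas.
; Shortly after BeginPlay, it also sends the dark message for components already inside the box.
; An IsNotATriggerCollider check gates each message, comparing component classes against box, sphere and trigger capsule types.
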(event OnComponentBeginOverlap(Box)
  (params (OverlappedComponent :type Primitive%20Component%20Object%20Reference) (OtherActor :type Actor%20Object%20Reference) (OtherComp :type Primitive%20Component%20Object%20Reference) (OtherBodyIndex :type Integer) (bFromSweep :type Boolean) (SweepResult :type Hit%20Result%20Structure%20%28by%20ref%29))
  (if (and (Utilities|IsNotATriggerCollider OtherComp) (Utilities|DoesObjectImplementInterface OtherActor "/Script/Scyther.CanEnterDarkLightAreas"))
    (Class|CanEnterDarkLightAreas|EnterDarkArea(Message) OtherActor)))

(event OnComponentEndOverlap(Box)
  (params (OverlappedComponent :type Primitive%20Component%20Object%20Reference) (OtherActor :type Actor%20Object%20Reference) (OtherComp :type Primitive%20Component%20Object%20Reference) (OtherBodyIndex :type Integer))
  (if (and (Utilities|IsNotATriggerCollider OtherComp) (Utilities|DoesObjectImplementInterface OtherActor "/Script/Scyther.CanEnterDarkLightAreas"))
    (Class|CanEnterDarkLightAreas|EnterLightArea(Message) OtherActor)))

(event EventBeginPlay
  (Utilities|FlowControl|Delay 0.2)
  (for _array_element (Class|PrimitiveComponent|GetOverlappingComponents (Variables|Default|GetBox))
    (if (and (Utilities|IsNotATriggerCollider _array_element) (Utilities|DoesObjectImplementInterface (Components|GetOwner _array_element) "/Script/Scyther.CanEnterDarkLightAreas"))
      (Class|CanEnterDarkLightAreas|EnterDarkArea(Message) (Components|GetOwner _array_element)))))

(fn ConstructionScript)