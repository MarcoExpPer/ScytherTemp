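; BP_DEBUGTIMER is a debug actor that measures how long the player stays inside its collision volume.
; Tick continuously adds delta seconds to a Time counter, whether or not the player is inside.
; Begin overlap from a component tagged PlayerBody resets the counter, and end overlap from one prints the elapsed time as a string.
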(event OnComponentBeginOverlap(CollisionComponent)
  (params (OverlappedComponent :type Primitive%20Component%20Object%20Reference) (OtherActor :type Actor%20Object%20Reference) (OtherComp :type Primitive%20Component%20Object%20Reference) (OtherBodyIndex :type Integer) (bFromSweep :type Boolean) (SweepResult :type Hit%20Result%20Structure%20%28by%20ref%29))
  (if (Components|ComponentHasTag OtherComp "PlayerBody")
    (Variables|Default|Settime 0.0)))

(event OnComponentEndOverlap(CollisionComponent)
  (params (OverlappedComponent :type Primitive%20Component%20Object%20Reference) (OtherActor :type Actor%20Object%20Reference) (OtherComp :type Primitive%20Component%20Object%20Reference) (OtherBodyIndex :type Integer))
  (if (Components|ComponentHasTag OtherComp "PlayerBody")
    (Development|PrintString (Utilities|String|ToString(Float) (Variables|Default|Gettime)))))

(event EventTick
  (params (DeltaSeconds :type Float%20%28single-precision%29))
  (bind _output_get (Variables|Default|Settime (+ (stale _output_get) DeltaSeconds))))

(fn ConstructionScript)