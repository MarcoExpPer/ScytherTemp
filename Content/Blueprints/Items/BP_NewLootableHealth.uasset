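; Health pickup that, when looted, flies toward the HUD health bar and then heals the player.
; On its looted event, if the UI animation is enabled, a timeline lerps the actor to a world point deprojected from the HP bar's screen position.
; When finished it hides, applies healing through the player's HealthComponent and self-destroys unless world-placed.
; Respawn stops the timeline before running the parent logic.
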(event Custom|startUIAnimation
  (bind _returnvalue (Game|GetPlayerController 0))
  (bind _real_hud (Variables|Default|GetReal%20Hud))
  (bind _ingame_wg (Variables|/Game/HUD/BluePrints/InGameHud/BP_InGameHud.BP_InGameHud_C|GetInGame_WG _real_hud))
  (bind _hpbar_background (Variables|/Game/HUD/BluePrints/InGameHud/WG_InGameUI.WG_InGameUI_C|GetHPBar_Background _ingame_wg))
  (bind _returnvalue_2 (Class|WidgetLayoutLibrary|SlotasCanvasSlot _hpbar_background))
  (bind _returnvalue_3 (Class|Widget|GetCachedGeometry _hpbar_background))
  (bind _returnvalue_4 (Class|CanvasPanelSlot|GetPosition _returnvalue_2))
  (bind _viewportposition (Class|SlateBlueprintLibrary|LocaltoViewport _returnvalue_3 _returnvalue_4))
  (bind _returnvalue_5 (- (.y _viewportposition) 1.0))
  (bind _returnvalue_6 (- (.x _viewportposition) 1.0))
  (bind (_worldlocation _worlddirection) (Class|PlayerController|DeprojectScreenPositiontoWorld _returnvalue _returnvalue_6 _returnvalue_5))
  (if (Variables|Default|GetdoUIAnimation)
    (Variables|Default|SetstartLocation (Transformation|GetActorLocation))
    (bind _newtrack_0 (Timeline|Timeline_0 Play)
      (:Update
        (Transformation|SetActorLocation (Math|Vector|Lerp(Vector) (Variables|Default|GetstartLocation) (+ _worldlocation (* _worlddirection 3.5e+03)) _newtrack_0) false false))
      (:Finished
        (Rendering|SetActorHiddenInGame true)
        (bind _asscyther_player_pawn (Utilities|Casting|CastToScytherPlayerPawn (Game|Player|GetPlayerPawn 0)))
        (Class|HealthComponent|ChangeHealth (Variables|/Script/Scyther.ScytherPlayerPawn|GethealthComponent _asscyther_player_pawn) (Variables|Default|GethealthAmount) "HEALING" true)
        (if (not (Variables|Default|GetisFromWorld))
          (Actor|DestroyActor))))))

(event EventBeginPlay
  (bind _asbp_in_game_hud (Utilities|Casting|CastToBP_InGameHud (HUD|GetHUD (Game|GetPlayerController 0))))
  (Variables|Default|SetReal%20Hud _asbp_in_game_hud)
  (EventDispatchers|BindEventtoLootedEvent (delegate Custom|startUIAnimation)))

(event EventRespawn
  (bind _returnvalue (Game|GetPlayerController 0))
  (bind _real_hud (Variables|Default|GetReal%20Hud))
  (bind _ingame_wg (Variables|/Game/HUD/BluePrints/InGameHud/BP_InGameHud.BP_InGameHud_C|GetInGame_WG _real_hud))
  (bind _hpbar_background (Variables|/Game/HUD/BluePrints/InGameHud/WG_InGameUI.WG_InGameUI_C|GetHPBar_Background _ingame_wg))
  (bind _returnvalue_2 (Class|WidgetLayoutLibrary|SlotasCanvasSlot _hpbar_background))
  (bind _returnvalue_3 (Class|Widget|GetCachedGeometry _hpbar_background))
  (bind _returnvalue_4 (Class|CanvasPanelSlot|GetPosition _returnvalue_2))
  (bind _viewportposition (Class|SlateBlueprintLibrary|LocaltoViewport _returnvalue_3 _returnvalue_4))
  (bind _returnvalue_5 (- (.y _viewportposition) 1.0))
  (bind _returnvalue_6 (- (.x _viewportposition) 1.0))
  (bind (_worldlocation _worlddirection) (Class|PlayerController|DeprojectScreenPositiontoWorld _returnvalue _returnvalue_6 _returnvalue_5))
  (Utilities|FlowControl|Sequence
    (:then_0
      (bind _newtrack_0 (Timeline|Timeline_0 Stop)
        (:Update
          (Transformation|SetActorLocation (Math|Vector|Lerp(Vector) (Variables|Default|GetstartLocation) (+ _worldlocation (* _worlddirection 3.5e+03)) _newtrack_0) false false))
        (:Finished
          (Rendering|SetActorHiddenInGame true)
          (bind _asscyther_player_pawn (Utilities|Casting|CastToScytherPlayerPawn (Game|Player|GetPlayerPawn 0)))
          (Class|HealthComponent|ChangeHealth (Variables|/Script/Scyther.ScytherPlayerPawn|GethealthComponent _asscyther_player_pawn) (Variables|Default|GethealthAmount) "HEALING" true)
          (if (not (Variables|Default|GetisFromWorld))
            (Actor|DestroyActor)))))
    (:then_1
      (|CallParentFunction))))

(fn ConstructionScript)