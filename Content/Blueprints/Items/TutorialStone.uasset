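; TutorialStone is a world prop whose mesh material switches between keyboard and gamepad variants to match the player's input device.
; On BeginPlay it binds to the BP_GameMode gamepad-usage update event and applies the current state.
; Later changes swap material slot 0 through UpdateMeshBasedOnKeyboard.
; The construction script defaults the mesh to the keyboard material.
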(event Custom|OnUsingGamepadChange
  (params (isUsingGamepad :type Boolean))
  (CallFunction|UpdateMeshBasedonKeyboard isUsingGamepad))

(event EventBeginPlay
  (bind _asbp_game_mode (Utilities|Casting|CastToBP_GameMode (Game|GetGameMode)))
  (EventDispatchers|BindEventtoIsUsingGamepadUpdated _asbp_game_mode (delegate Custom|OnUsingGamepadChange))
  (CallFunction|UpdateMeshBasedonKeyboard (Variables|/Game/Blueprints/Managers/BP_GameMode.BP_GameMode_C|GetisUsingGamepad? _asbp_game_mode)))

(event Collision|EventActorBeginOverlap
  (params (OtherActor :type Actor%20Object%20Reference)))

(event EventTick
  (params (DeltaSeconds :type Float%20%28single-precision%29)))

(fn ConstructionScript
  (Rendering|Material|SetMaterial (Variables|Default|GetStaticMesh) 0 (Variables|Default|GetkeyboardMat)))

(fn UpdateMeshBasedonKeyboard
  (params (isUsingGamepad :type Boolean))
  (Rendering|Material|SetMaterial (Variables|Default|GetStaticMesh) 0 (select isUsingGamepad (Variables|Default|GetGamepadMat) (Variables|Default|GetkeyboardMat))))