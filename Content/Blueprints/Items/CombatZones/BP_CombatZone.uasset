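; BP_CombatZone is a combat zone that propagates combat start, end and respawn to its SubCombatZones.
; At BeginPlay, RespawnType decides whether it destroys itself and its sub-zones when combat ends or stays respawnable.
; Respawnable zones register with the game mode's RespawnMan at combat start, in either the always-respawn or until-checkpoint list.
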(event Custom|CombatStartsEvent_Event_0
  (bind _self self)
  (Utilities|FlowControl|Sequence
    (:then_0
      (bind _asscyther_game_mode_base (Utilities|Casting|CastToScytherGameModeBase (Game|GetGameMode)))
      (if (Utilities|Enum|Equal(Enum) (Variables|CombatZone|GetRespawnType) "NewEnumerator0")
        (Class|RespawnManager|AddtoAlwaysRespawnList (Variables|/Script/Scyther.ScytherGameModeBase|GetrespawnMan _asscyther_game_mode_base) _self)
        (else
          (Class|RespawnManager|AddtoRespawnUntilCheckpointList (Variables|/Script/Scyther.ScytherGameModeBase|GetrespawnMan _asscyther_game_mode_base) _self))))
    (:then_1
      (for _array_element (Variables|Default|GetsubCombatZones)
        (Class|CombatZone|StartCombat _array_element)))))

(event Custom|CombatEndsEvent_Event_0
  (Actor|DestroyActor)
  (for _array_element (Variables|Default|GetsubCombatZones)
    (Actor|DestroyActor _array_element)))

(event Custom|CustomEvent_0
  (for _array_element (Variables|Default|GetsubCombatZones)
    (Class|CombatZone|EndCombat _array_element false)))

(event EventBeginPlay
  (if (Utilities|Enum|Equal(Enum) (Variables|CombatZone|GetRespawnType) "NewEnumerator2")
    (EventDispatchers|AssignCombatEndsEvent (delegate Custom|CombatEndsEvent_Event_0))
    (else
      (EventDispatchers|AssignCombatStartsEvent (delegate Custom|CombatStartsEvent_Event_0))
      (EventDispatchers|BindEventtoCombatEndsEvent (delegate Custom|CustomEvent_0)))))

(event EventRespawn
  (Class|CombatZone|RespawnCombatZone)
  (for _array_element (Variables|Default|GetsubCombatZones)
    (Class|CanRespawn|Respawn _array_element)))

(fn ConstructionScript)