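; Combat zone door that shatters when told to close, using a destructible mesh.
; Opening or preparing rebuilds the mesh by clearing and reassigning it, moves it to an offset from the actor, and restores collision and opacity.
; Closing explodes it with radius damage, disables collision and starts a despawn timer.
; The timer runs a timeline driving material opacity, and reopening cancels both timer and timeline.
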(event Custom|Hide
  (bind _newtrack_0 (Timeline|Timeline_0 PlayFromStart)
    (:Update
      (Rendering|Material|SetScalarParameterValueonMaterials (Variables|Default|GetDestructible) "Opacity" _newtrack_0))))

(event Custom|StopTimeline
  (bind _newtrack_0 (Timeline|Timeline_0 Stop)
    (:Update
      (Rendering|Material|SetScalarParameterValueonMaterials (Variables|Default|GetDestructible) "Opacity" _newtrack_0))))

(event EventBeginPlay
  (bind _returnvalue (Class|DestructibleComponent|GetDestructibleMesh (Variables|Default|GetDestructible)))
  (Variables|Default|SetDM_Class (Utilities|GetClass _returnvalue))
  (Variables|Default|SetinitialTransform (Transformation|GetActorTransform)))

(event EventPrepareCombatZoneDoor
  (CallFunction|RespawnDestructible)
  (CallFunction|MoveDoortoOpenPosition)
  (Rendering|SetVisibility (Variables|Default|GetDestructible) true false)
  (Collision|SetCollisionEnabled (Variables|Default|GetBox) "QueryAndPhysics")
  (Utilities|Time|ClearandInvalidateTimerbyHandle (Variables|Default|GetNewVar_0))
  (CallFunction|StopTimeline)
  (Rendering|Material|SetScalarParameterValueonMaterials (Variables|Default|GetDestructible) "Opacity" 1.0))

(event EventTick
  (params (DeltaSeconds :type Float%20%28single-precision%29)))

(event EventOpenCombatZoneDoor
  (CallFunction|RespawnDestructible)
  (CallFunction|MoveDoortoOpenPosition)
  (Rendering|SetVisibility (Variables|Default|GetDestructible) true false)
  (Collision|SetCollisionEnabled (Variables|Default|GetBox) "QueryAndPhysics")
  (Utilities|Time|ClearandInvalidateTimerbyHandle (Variables|Default|GetNewVar_0))
  (CallFunction|StopTimeline)
  (Rendering|Material|SetScalarParameterValueonMaterials (Variables|Default|GetDestructible) "Opacity" 1.0))

(event EventCloseCombatZoneDoor
  (CallFunction|ExplodeDestructible)
  (Collision|SetCollisionEnabled (Variables|Default|GetBox) "NoCollision")
  (bind _returnvalue (Utilities|Time|SetTimerbyEvent (delegate Custom|Hide) (Variables|Default|GettimeToDespawn)))
  (Variables|Default|SetNewVar_0 _returnvalue))

(fn ConstructionScript)

(fn ExplodeDestructible
  (Collision|SetCollisionProfileName (Variables|Default|GetDestructible) "Destructible" true :!class /Script/Engine.PrimitiveComponent)
  (Class|DestructibleComponent|ApplyRadiusDamage (Variables|Default|GetDestructible) 1.0 (Transformation|GetActorLocation) (Variables|Default|GetDamage%20Radius) (Variables|Default|GetImpulse%20Strength) true)
  (return))

(fn RebuildDestructible)

(fn MoveDoortoOpenPosition
  (bind _returnvalue (Transformation|GetActorLocation))
  (Variables|Default|SetclosedLocation _returnvalue)
  (Transformation|SetWorldLocation (Variables|Default|GetDestructible) (+ _returnvalue (Variables|Default|GetinitialOpenOffset)) false true))

(fn RespawnDestructible
  (bind _destructible (Variables|Default|GetDestructible))
  (bind _returnvalue (Class|DestructibleComponent|GetDestructibleMesh _destructible))
  (LocalVariables|SetNewMesh _returnvalue)
  (Class|DestructibleComponent|SetDestructibleMesh _destructible)
  (Class|DestructibleComponent|SetDestructibleMesh (Variables|Default|GetDestructible) (LocalVariables|GetNewMesh)))