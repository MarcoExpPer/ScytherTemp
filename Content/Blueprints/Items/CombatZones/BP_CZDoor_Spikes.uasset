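; Combat zone door (spikes variant) built on a destructible mesh that blocks while closed and shatters when opened.
; Prepare respawns the mesh by clearing and reassigning it, then parks it at an offset without collision; Close enables collision and lerps it into place.
; Open disables collision, breaks the mesh with radial damage, plays a breaking sound event, then after a delay animates material opacity to fade the debris.
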(event Custom|CustomEvent_0
  (bind _newtrack_0 (Timeline|Timeline_1 PlayFromStart)
    (:Update
      (Rendering|Material|SetScalarParameterValueonMaterials (Variables|Default|GetDestructible) "Opacity" _newtrack_0))))

(event Custom|StopTimeLine
  (bind _newtrack_0 (Timeline|Timeline_1 Stop)
    (:Update
      (Rendering|Material|SetScalarParameterValueonMaterials (Variables|Default|GetDestructible) "Opacity" _newtrack_0))))

(event EventBeginPlay
  (bind _returnvalue (Class|DestructibleComponent|GetDestructibleMesh (Variables|Default|GetDestructible)))
  (Variables|Default|SetDM_Class (Utilities|GetClass _returnvalue))
  (Variables|Default|SetinitialTransform (Transformation|GetActorTransform)))

(event EventPrepareCombatZoneDoor
  (bind _closedlocation (Variables|Default|GetclosedLocation))
  (Utilities|FlowControl|Sequence
    (:then_0
      (bind _newtrack_0 (Timeline|Timeline_0 Stop)
        (:Update
          (Transformation|SetWorldLocation (Variables|Default|GetDestructible) (Math|Vector|Lerp(Vector) (+ _closedlocation (Variables|Default|GetinitialOpenOffset)) _closedlocation _newtrack_0) false false))))
    (:then_1
      (Utilities|Time|ClearandInvalidateTimerbyHandle (Variables|Default|GetHideVisibilityTimerHandle))
      (CallFunction|RespawnDestructible)
      (CallFunction|MoveDoortoOpenPosition)
      (Collision|SetCollisionEnabled (Variables|Default|GetBox) "NoCollision")
      (Rendering|SetVisibility (Variables|Default|GetDestructible) true true)
      (CallFunction|StopTimeLine)
      (Rendering|Material|SetScalarParameterValueonMaterials (Variables|Default|GetDestructible) "Opacity" 1.0))))

(event EventTick
  (params (DeltaSeconds :type Float%20%28single-precision%29)))

(event EventOpenCombatZoneDoor
  (Collision|SetCollisionEnabled (Variables|Default|GetBox) "NoCollision")
  (CallFunction|ExplodeDestructible)
  (bind _returnvalue (Utilities|Time|SetTimerbyEvent (delegate Custom|CustomEvent_0) (Variables|Default|GettimeToDespawn)))
  (Variables|Default|SetHideVisibilityTimerHandle _returnvalue))

(event EventCloseCombatZoneDoor
  (bind _closedlocation (Variables|Default|GetclosedLocation))
  (Collision|SetCollisionEnabled (Variables|Default|GetBox) "QueryAndPhysics")
  (Rendering|SetVisibility (Variables|Default|GetDestructible) true false)
  (bind _newtrack_0 (Timeline|Timeline_0 PlayFromStart)
    (:Update
      (Transformation|SetWorldLocation (Variables|Default|GetDestructible) (Math|Vector|Lerp(Vector) (+ _closedlocation (Variables|Default|GetinitialOpenOffset)) _closedlocation _newtrack_0) false false))))

(fn ConstructionScript)

(fn ExplodeDestructible
  (bind _returnvalue (Transformation|GetActorLocation))
  (Collision|SetCollisionProfileName (Variables|Default|GetDestructible) "Destructible" true :!class /Script/Engine.PrimitiveComponent)
  (Class|DestructibleComponent|ApplyRadiusDamage (Variables|Default|GetDestructible) 1.0 _returnvalue (Variables|Default|GetDamage%20Radius) (Variables|Default|GetImpulse%20Strength) true)
  (Class|FMODBlueprintStatics|PlayEventatLocation "/Game/FMOD/Events/Enviroment/SFX/SFX_Breaking_Things/BreakingCombatZone.BreakingCombatZone" (Math|Conversions|ToTransform(Vector) _returnvalue))
  (return))

(fn MoveDoortoOpenPosition
  (bind _returnvalue (Transformation|GetActorLocation))
  (Variables|Default|SetclosedLocation _returnvalue)
  (Transformation|SetWorldLocation (Variables|Default|GetDestructible) (+ _returnvalue (Variables|Default|GetinitialOpenOffset)) false true))

(fn RespawnDestructible
  (bind _destructible (Variables|Default|GetDestructible))
  (bind _returnvalue (Class|DestructibleComponent|GetDestructibleMesh _destructible))
  (LocalVariables|SetNewMesh _returnvalue)
  (Class|DestructibleComponent|SetDestructibleMesh _destructible)
  (Class|DestructibleComponent|SetDestructibleMesh (Variables|Default|GetDestructible) (LocalVariables|GetNewMesh)))