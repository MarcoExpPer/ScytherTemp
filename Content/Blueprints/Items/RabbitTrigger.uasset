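; RabbitTrigger is a box trigger that despawns or teleports one designated enemy when that enemy's body enters it.
; On overlap it checks for EnemyThatWillTrigger and the EnemyBody tag, then either calls DeSpawn or, if teleporting is enabled, runs TeleportEnemy.
; TeleportEnemy moves the enemy to a set world location, printing an error if that location is zero.
; The option to force a change to dark is stubbed and does nothing.
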(event OnComponentBeginOverlap(Box)
  (params (OverlappedComponent :type Primitive%20Component%20Object%20Reference) (OtherActor :type Actor%20Object%20Reference) (OtherComp :type Primitive%20Component%20Object%20Reference) (OtherBodyIndex :type Integer) (bFromSweep :type Boolean) (SweepResult :type Hit%20Result%20Structure%20%28by%20ref%29))
  (if (and (== OtherActor (Variables|Default|GetEnemyThatWillTrigger)) (Components|ComponentHasTag OtherComp "EnemyBody"))
    (if (Variables|Default|GetDespawnEnemy?)
      (Class|BaseEnemy|DeSpawn (Variables|Default|GetEnemyThatWillTrigger))
      (elif (Variables|Default|GetIsTeleporting?)
        (CallFunction|TeleportEnemy)
        (if (Variables|Default|GetisForcingChangeToDark?)
          _)))))

(event EventBeginPlay)

(event Collision|EventActorBeginOverlap
  (params (OtherActor :type Actor%20Object%20Reference)))

(event EventTick
  (params (DeltaSeconds :type Float%20%28single-precision%29)))

(fn ConstructionScript)

(fn TeleportEnemy
  (if (Math|Vector|Equal(Vector) (Variables|Default|GetWorldLocationToTeleportTo) "0, 0, 0" 0.0001)
    (Development|PrintString "Location to teleport to is invalid")
    (return)
    (else
      (bind _returnvalue (Transformation|SetActorLocation (Variables|Default|GetEnemyThatWillTrigger) (Variables|Default|GetWorldLocationToTeleportTo) false true))
      (if _returnvalue
        (return)))))

(fn ForceEnemytoDark)