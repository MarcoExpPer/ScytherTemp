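; Player pawn Blueprint for Scyther that keeps a PositionMarker component on the static world surface below it.
; Every tick it line-traces 1000 units straight down against WorldStatic objects, ignoring itself, and moves the marker to the impact point.
; The hit result is not checked before the marker moves, and the other events and construction script are empty.
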(event EventBeginPlay)

(event Collision|EventActorBeginOverlap
  (params (OtherActor :type Actor%20Object%20Reference)))

(event EventTick
  (params (DeltaSeconds :type Float%20%28single-precision%29))
  (bind _returnvalue (Transformation|GetActorLocation))
  (bind _outhit (Collision|LineTraceForObjects _returnvalue (+ _returnvalue (* (Math|Vector|VectorDown) 1e+03)) (Utilities|Array|MakeArray "ObjectTypeQuery1") false (Utilities|Array|MakeArray self) "None" true "(R=1.000000,G=0.000000,B=0.000000,A=1.000000)" "(R=0.000000,G=1.000000,B=0.000000,A=1.000000)" 0.0))
  (Transformation|SetWorldLocation (Variables|Default|GetPositionMarker) (.ImpactPoint (Collision|BreakHitResult _outhit)) false false))

(fn ConstructionScript)