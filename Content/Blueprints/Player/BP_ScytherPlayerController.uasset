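; Player controller for the Scyther player that handles hardcoded skill hotkeys and input-device detection.
; BeginPlay sets game-only input and caches the player pawn and BP_GameMode.
; H enables the combined skill on the pawn's SkillComponent, while L and K update its light and non-light mana by a fixed amount.
; Every key press tells the game mode whether a gamepad is in use.
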(event EventBeginPlay
  (Utilities|FlowControl|Sequence
    (:then_0
      (Input|SetInputModeGameOnly (Game|GetPlayerController 0))
      (bind _asbp_scyther_player_pawn (Utilities|Casting|CastToBP_ScytherPlayerPawn (Game|Player|GetPlayerPawn 0)))
      (bind _output_get (Variables|Default|SetAs%20BP%20Scyther%20Player%20Pawn _asbp_scyther_player_pawn)))
    (:then_1
      (bind _asbp_game_mode (Utilities|Casting|CastToBP_GameMode (Game|GetGameMode)))
      (Variables|Default|SetAs%20BP%20Game%20Mode _asbp_game_mode))))

(event EventTick
  (params (DeltaSeconds :type Float%20%28single-precision%29)))

(event Input|KeyboardEvents|L
  (params (Key :type Key%20Structure :default "None"))
  (:Pressed
    (Class|SkillComponent|UpdateMana (Variables|/Script/Scyther.ScytherPlayerPawn|GetskillComponent (stale EventBeginPlay _output_get)) true 1e+01)))

(event Input|KeyboardEvents|AnyKey
  (params (Key :type Key%20Structure :default "None"))
  (:Pressed
    (Default|ChangeIsUsingGamepad (Variables|Default|GetAs%20BP%20Game%20Mode) (Class|KismetInputLibrary|KeyIsGamepadKey Key))))

(event Input|KeyboardEvents|H
  (params (Key :type Key%20Structure :default "None"))
  (:Pressed
    (Class|SkillComponent|EnabledCombinedSkill (Variables|/Script/Scyther.ScytherPlayerPawn|GetskillComponent (stale EventBeginPlay _output_get)))))

(event Input|KeyboardEvents|K
  (params (Key :type Key%20Structure :default "None"))
  (:Pressed
    (Class|SkillComponent|UpdateMana (Variables|/Script/Scyther.ScytherPlayerPawn|GetskillComponent (stale EventBeginPlay _output_get)) false 1e+01)))

(fn ConstructionScript)