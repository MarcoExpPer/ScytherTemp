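; BP_CameraRail is a rail camera that follows the player along a referenced spline, starting on BeginPlay if marked main.
; ActivateCamera blends the view to it and enables movement, which StopCamera disables.
; Each Tick, both movement modes take X from the player minus an offset and Y/Z from the nearest spline point, despite MoveDepth's differing comment.
; Depth mode also lerps camera rotation by clamped player distance.
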(event Custom|StopCamera
  (Variables|Default|SetallowMovement false))

(event Custom|ActivateCamera
  (params (blendTime :type Float%20%28single-precision%29))
  (Variables|Default|SetallowMovement true)
  (Game|Player|SetViewTargetwithBlend (Game|GetPlayerController 0) self blendTime "VTBlend_Linear" 0.0 false))

(event EventBeginPlay
  (if (Variables|Default|GetisMainCamera?)
    (CallFunction|ActivateCamera 1.0)))

(event EventTick
  (params (DeltaSeconds :type Float%20%28single-precision%29))
  (if (Variables|Default|GetallowMovement)
    (switch Utilities|FlowControl|Switch|SwitchonCameraMovementType (Variables|Default|GetcameraMovementType)
      (:NewEnumerator0
        (CallFunction|MoveDepth))
      (:NewEnumerator1
        (CallFunction|MoveRight/Left)))))

(fn ConstructionScript)

(fn MoveRight/Left
  (bind _returnvalue (Transformation|GetActorLocation))
  (bind _splineref (Variables|Default|GetsplineRef))
  (bind _spline (Variables|/Game/Blueprints/Player/Camera/BP_CameraSpline.BP_CameraSpline_C|GetSpline _splineref))
  (bind _returnvalue_2 (Spline|FindLocationClosesttoWorldLocation _spline _returnvalue "World"))
  ;[1 1 1] The player decides the X location of the camera
  (Transformation|SetActorLocation (Math|Vector|MakeVector (- (.x (Transformation|GetActorLocation (Game|Player|GetPlayerPawn 0))) (Variables|Default|GetPlayerOffset)) (.y _returnvalue_2) (.z _returnvalue_2)) false false))

(fn MoveDepth
  (bind _returnvalue (Transformation|GetActorLocation))
  (bind _splineref (Variables|Default|GetsplineRef))
  (bind _spline (Variables|/Game/Blueprints/Player/Camera/BP_CameraSpline.BP_CameraSpline_C|GetSpline _splineref))
  (bind _returnvalue_2 (Spline|FindLocationClosesttoWorldLocation _spline _returnvalue "World"))
  ;[1 1 1] The player decides the Y location of the camera
  (Transformation|SetActorLocation (Math|Vector|MakeVector (- (.x (Transformation|GetActorLocation (Game|Player|GetPlayerPawn 0))) (Variables|Default|GetPlayerOffset)) (.y _returnvalue_2) (.z _returnvalue_2)) false false)
  (Transformation|SetActorRotation (Math|Rotator|Lerp(Rotator) (Variables|Rotation|GetmaxRotation) (Variables|Rotation|GetminRotation) (/ (Math|Float|Max(Float) (Math|Float|Min(Float) (Math|Vector|Distance(Vector) (Transformation|GetActorLocation) (Transformation|GetActorLocation (Game|Player|GetPlayerPawn 0))) (Variables|Rotation|GetmaxRotationDistance)) (Variables|Rotation|GetminRotationDistance)) (- (Variables|Rotation|GetmaxRotationDistance) (Variables|Rotation|GetminRotationDistance))))))