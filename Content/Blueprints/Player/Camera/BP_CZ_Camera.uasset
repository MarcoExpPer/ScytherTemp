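; BP_CZ_Camera is a combat zone camera that can take over the player's view from the rail camera during combat.
; It caches the BP_ScytherPlayerController shortly after BeginPlay to reach its RailCamera.
; When its CombatZone starts combat, it stops the rail camera and blends the view target to itself.
; When combat ends, it reactivates the rail camera with the same blend time; both handoffs require the ActivateCamera flag.
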(event CombatStartsEvent(CombatZone)
  (if (Variables|Default|GetactivateCamera?)
    (Default|StopCamera (Variables|/Game/Blueprints/Player/BP_ScytherPlayerController.BP_ScytherPlayerController_C|GetrailCamera (Variables|Default|GetAs%20BP%20Scyther%20Player%20Controller)))
    (CallFunction|ActivateCamera (Variables|Default|GetblendTime))))

(event CombatEndsEvent(CombatZone)
  (if (Variables|Default|GetactivateCamera?)
    (Default|ActivateCamera (Variables|/Game/Blueprints/Player/BP_ScytherPlayerController.BP_ScytherPlayerController_C|GetrailCamera (Variables|Default|GetAs%20BP%20Scyther%20Player%20Controller)) (Variables|Default|GetblendTime))))

(event EventBeginPlay
  (Utilities|FlowControl|Delay 0.2)
  (bind _asbp_scyther_player_controller (Utilities|Casting|CastToBP_ScytherPlayerController (Game|GetPlayerController 0)))
  (Variables|Default|SetAs%20BP%20Scyther%20Player%20Controller _asbp_scyther_player_controller))

(fn ConstructionScript)

(fn ActivateCamera
  (params (blendTime1 :type Float%20%28single-precision%29))
  (Game|Player|SetViewTargetwithBlend (Game|GetPlayerController 0) self blendTime1 "VTBlend_Linear" 0.0 false))