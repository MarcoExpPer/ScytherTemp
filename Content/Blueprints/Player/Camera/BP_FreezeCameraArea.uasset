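; Trigger volume that blends the view to its own fixed camera while the player body is inside, and back to the main camera on exit.
; Box overlaps on PlayerBody-tagged components drive the enter and exit switches, which are ignored while a blend runs.
; A timer ends each blend and rechecks the player's position, catching crossings made mid-blend.
; Player respawn clears the timers and instantly restores the main camera.
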(event OnComponentBeginOverlap(Box)
  (params (OverlappedComponent :type Primitive%20Component%20Object%20Reference) (OtherActor :type Actor%20Object%20Reference) (OtherComp :type Primitive%20Component%20Object%20Reference) (OtherBodyIndex :type Integer) (bFromSweep :type Boolean) (SweepResult :type Hit%20Result%20Structure%20%28by%20ref%29))
  (if (Components|ComponentHasTag OtherComp "PlayerBody")
    (Variables|Default|SetisPlayerInside? true)
    (if (Math|Boolean|ANDBoolean (not (Variables|Default|GetisBlending)) (not (Variables|Default|GetisFixedCameraActive?)) (Variables|Default|GetisPlayerInside?))
      (Variables|Default|SetisFixedCameraActive? true)
      (Default|StopCamera (Variables|Default|GetMainCamera))
      (CallFunction|ActivateCamera (Variables|Default|GetblendTime)))))

(event OnComponentEndOverlap(Box)
  (params (OverlappedComponent :type Primitive%20Component%20Object%20Reference) (OtherActor :type Actor%20Object%20Reference) (OtherComp :type Primitive%20Component%20Object%20Reference) (OtherBodyIndex :type Integer))
  (bind _blendtime (Variables|Default|GetblendTime))
  (if (Components|ComponentHasTag OtherComp "PlayerBody")
    (Variables|Default|SetisPlayerInside? false)
    (if (Math|Boolean|ANDBoolean (not (Variables|Default|GetisBlending)) (Variables|Default|GetisFixedCameraActive?) (not (Variables|Default|GetisPlayerInside?)))
      (Utilities|Time|ClearandInvalidateTimerbyHandle (Variables|Default|GetactivateFixedCameraHandle))
      (Variables|Default|SetisFixedCameraActive? false)
      (Variables|Default|SetisBlending true)
      (Default|ActivateCamera (Variables|Default|GetMainCamera) _blendtime)
      (Utilities|Time|ClearandInvalidateTimerbyHandle (Variables|Default|GetactivateMainCameraHandle))
      (bind _returnvalue (Utilities|Time|SetTimerbyEvent (delegate Custom|MainCameraActivationFinished) _blendtime))
      (Variables|Default|SetactivateMainCameraHandle _returnvalue))))

(event Custom|TriggerPlayerEnter
  (if (Math|Boolean|ANDBoolean (not (Variables|Default|GetisBlending)) (not (Variables|Default|GetisFixedCameraActive?)) (Variables|Default|GetisPlayerInside?))
    (Variables|Default|SetisFixedCameraActive? true)
    (Default|StopCamera (Variables|Default|GetMainCamera))
    (CallFunction|ActivateCamera (Variables|Default|GetblendTime))))

(event Custom|TriggerPlayerExits
  (bind _blendtime (Variables|Default|GetblendTime))
  (if (Math|Boolean|ANDBoolean (not (Variables|Default|GetisBlending)) (Variables|Default|GetisFixedCameraActive?) (not (Variables|Default|GetisPlayerInside?)))
    (Utilities|Time|ClearandInvalidateTimerbyHandle (Variables|Default|GetactivateFixedCameraHandle))
    (Variables|Default|SetisFixedCameraActive? false)
    (Variables|Default|SetisBlending true)
    (Default|ActivateCamera (Variables|Default|GetMainCamera) _blendtime)
    (Utilities|Time|ClearandInvalidateTimerbyHandle (Variables|Default|GetactivateMainCameraHandle))
    (bind _returnvalue (Utilities|Time|SetTimerbyEvent (delegate Custom|MainCameraActivationFinished) _blendtime))
    (Variables|Default|SetactivateMainCameraHandle _returnvalue)))

(event Custom|MainCameraActivationFinished
  (Variables|Default|SetisBlending false)
  (CallFunction|TriggerPlayerEnter))

(event Custom|ActivateCamera
  (params (blendTime :type Float%20%28single-precision%29))
  (Utilities|Time|ClearandInvalidateTimerbyHandle (Variables|Default|GetactivateMainCameraHandle))
  (Game|Player|SetViewTargetwithBlend (Game|GetPlayerController 0) self blendTime "VTBlend_Linear" 0.0 false)
  (Variables|Default|SetisBlending true)
  (Utilities|Time|ClearandInvalidateTimerbyHandle (Variables|Default|GetactivateFixedCameraHandle))
  (bind _returnvalue (Utilities|Time|SetTimerbyEvent (delegate Custom|CustomEvent_0) blendTime))
  (Variables|Default|SetactivateFixedCameraHandle _returnvalue))

(event Custom|CustomEvent_0
  (Variables|Default|SetisBlending false)
  (CallFunction|TriggerPlayerExits))

(event Custom|CustomEvent_1
  (params (location :type Vector))
  (Utilities|Time|ClearandInvalidateTimerbyHandle (Variables|Default|GetactivateFixedCameraHandle))
  (Utilities|Time|ClearandInvalidateTimerbyHandle (Variables|Default|GetactivateMainCameraHandle))
  (Default|ActivateCamera (Variables|Default|GetMainCamera) 0.0)
  (Variables|Default|SetisFixedCameraActive? false)
  (Variables|Default|SetisPlayerInside? false)
  (Variables|Default|SetisBlending false))

(event EventBeginPlay
  (bind _asscyther_player_controller (Utilities|Casting|CastToScytherPlayerController (Game|GetPlayerController 0)))
  (Variables|Default|SetAs%20BP%20Player%20Controller _asscyther_player_controller)
  (Variables|Default|SetisBlending false)
  (bind _asbp_game_mode (Utilities|Casting|CastToBP_GameMode (Game|GetGameMode)))
  (Utilities|FlowControl|Delay 0.2)
  (EventDispatchers|BindEventtoPlayerRespawnEvent (Variables|/Script/Scyther.ScytherGameModeBase|GetrespawnMan _asbp_game_mode) (delegate Custom|CustomEvent_1)))

(fn ConstructionScript)