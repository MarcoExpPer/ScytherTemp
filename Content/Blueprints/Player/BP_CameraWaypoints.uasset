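; Side-scrolling camera actor that becomes player 0's view target and tracks the character along Y on a waypoint-defined path.
; Each tick, UpdateWaypoints shifts the active index pair as the camera crosses waypoint Y bounds.
; X and Z are lerped between that pair using squared-distance ratios to the right waypoint.
; The actor also tilts slightly with the player's X depth from the start, and prints the left index for debugging.
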(event EventBeginPlay
  (Game|Player|SetViewTargetwithBlend (Game|GetPlayerController 0) self 0.0 "VTBlend_Linear" 0.0 false)
  (Transformation|SetRelativeRotation (Variables|CameraActor|GetCameraComponent) "-15.000000,0.000000, 0" false false)
  (Variables|Default|SetinitialPlayerLocation (Transformation|GetActorLocation (Game|GetPlayerCharacter 0)))
  (Variables|Default|SetleftWaypoint 0)
  (Variables|Default|SetrightWaypoint 1))

(event Collision|EventActorBeginOverlap
  (params (OtherActor :type Actor%20Object%20Reference)))

(event EventTick
  (params (DeltaSeconds :type Float%20%28single-precision%29))
  (bind _returnvalue (Transformation|GetActorLocation))
  (bind _waypoints (Variables|Default|Getwaypoints))
  (bind _waypoints_2 (Variables|Default|Getwaypoints))
  (bind _leftwaypoint (Variables|Default|GetleftWaypoint))
  (bind _rightwaypoint (Variables|Default|GetrightWaypoint))
  (bind _output (Utilities|Array|Get(acopy) _waypoints _rightwaypoint))
  (bind _output_2 (Utilities|Array|Get(acopy) _waypoints_2 _leftwaypoint))
  (bind _returnvalue_2 (Transformation|GetActorLocation _output))
  (bind _returnvalue_3 (Transformation|GetActorLocation _output_2))
  (bind _returnvalue_4 (Class|KismetMathLibrary|VectorDistanceSquared _returnvalue _returnvalue_2))
  (bind _returnvalue_5 (Class|KismetMathLibrary|VectorDistanceSquared _returnvalue_3 _returnvalue_2))
  (bind _returnvalue_6 (/ _returnvalue_4 _returnvalue_5))
  (bind _returnvalue_7 (Math|Vector|Lerp(Vector) _returnvalue_3 _returnvalue_2 _returnvalue_6))
  (Transformation|SetActorRotation (Math|Rotator|Lerp(Rotator) "0.000000,180.000000, 0" "5.000000,180.000000, 0" (/ (Math|Float|Clamp(Float) (- (.x (Variables|Default|GetinitialPlayerLocation)) (.x (Transformation|GetActorLocation (Game|GetPlayerCharacter 0)))) 0.0 (Variables|Default|GetmaxDepth)) (Variables|Default|GetmaxDepth))))
  (CallFunction|UpdateWaypoints)
  (Transformation|SetActorLocation (Math|Vector|MakeVector (.x _returnvalue_7) (.y (Transformation|GetActorLocation (Game|GetPlayerCharacter 0))) (.z _returnvalue_7)) false false)
  (Development|PrintString (Utilities|String|ToString(Integer) (Variables|Default|GetleftWaypoint))))

(fn ConstructionScript)

(fn UpdateWaypoints
  (if (> (.y (Transformation|GetActorLocation)) (.y (Transformation|GetActorLocation (Utilities|Array|Get(acopy) (Variables|Default|Getwaypoints) (Variables|Default|GetleftWaypoint)))))
    ;[1 1 1] Si ya estamos en el limite izq, no hacemos nada
    (if (not (== (Variables|Default|GetleftWaypoint) 0))
      ;[1 1 1] Movemos los waypoints actuales a la izq
      (Math|Integer|DecrementInt (Variables|Default|GetrightWaypoint)
        (:%20%20
          (Math|Integer|DecrementInt (Variables|Default|GetleftWaypoint)
            (:%20%20
              (return))))))
    (elif (< (.y (Transformation|GetActorLocation)) (.y (Transformation|GetActorLocation (Utilities|Array|Get(acopy) (Variables|Default|Getwaypoints) (Variables|Default|GetrightWaypoint)))))
      (if (== (Variables|Default|GetleftWaypoint) (- (Utilities|Array|Length (Variables|Default|Getwaypoints)) 1))
        (return)
        (else
          ;[1 1 1] Movemos los waypoints actuales a la der
          (Math|Integer|IncrementInt (Variables|Default|GetrightWaypoint)
            (:%20%20
              (Math|Integer|IncrementInt (Variables|Default|GetleftWaypoint)
                (:%20%20
                  (return)))))))
      (else
        (return)))))