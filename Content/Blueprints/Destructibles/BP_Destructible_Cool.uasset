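; Destructible prop that plays hit sound and force feedback when damaged, then shatters and drops loot at zero health if destructible.
; Breaking applies radius damage to the destructible mesh and traces down to limit loot drop height.
; Respawn type either destroys the actor or registers it with the game mode's respawn manager and fades debris after a timer.
; Respawn restores health, transform, collision and opacity, clearing and reassigning the mesh to undo fracturing.
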(event HealthChangedEvent(Health)
  (params (oldHp :type Float%20%28single-precision%29) (newHp :type Float%20%28single-precision%29) (damageType :type DamageModes%20Enum :default "DASHEABLE"))
  (if (< newHp oldHp)
    (CallFunction|DoHitSound)
    (CallFunction|DoForceEffect)))

(event ZerohealthEvent(Health)
  (params (damageType :type DamageModes%20Enum :default "DASHEABLE"))
  (if (Variables|Diseño|GetIsDestruible)
    (CallFunction|DestroyDestructible)
    (else
      (CallFunction|DoHitSound))))

(event Custom|Initialize
  (bind _box (Variables|Default|GetBox))
  (if (Variables|Diseño|GethasCollision?)
    (Collision|SetCollisionResponsetoAllChannels _box "ECR_Block")
    (Collision|SetCollisionResponsetoChannel _box "ECC_Visibility" "ECR_Ignore")
    (else
      (Collision|SetCollisionObjectType (Variables|Default|GetBox) "ECC_WorldDynamic")
      (Collision|SetCollisionResponsetoAllChannels (Variables|Default|GetBox) "ECR_Overlap")))
  (if (Variables|Diseño|GetcanPlayerStepOn?)
    (Collision|SetCollisionObjectType (Variables|Default|GetBox) "ECC_WorldStatic")))

(event Custom|Hide
  (bind _newtrack_0 (Timeline|Timeline_0 PlayFromStart)
    (:Update
      (Rendering|Material|SetScalarParameterValueonMaterials (Variables|Default|GetDestructible1) "Opacity" _newtrack_0))))

(event Custom|DestroyDestructible
  (bind _self self)
  (bind _scythergamemode (Variables|Default|GetScytherGameMode))
  (bind _respawnman (Variables|/Script/Scyther.ScytherGameModeBase|GetrespawnMan _scythergamemode))
  (Components|Activation|Deactivate (Variables|Default|GetNiagara))
  (Collision|SetCollisionEnabled (Variables|Default|GetDestructible1) "QueryAndPhysics")
  (if (Variables|Default|GetDoOnBreakSound)
    (CallFunction|DestroySound))
  (Variables|Default|SetLooteableOrigin (.Origin (Collision|GetActorBounds false false)))
  (bind _outhit (Collision|LineTraceByChannel (Variables|Default|GetLooteableOrigin) (+ (Variables|Default|GetLooteableOrigin) (* (Math|Vector|VectorDown) 1e+03)) "TraceTypeQuery1" false 0 "None" true "(R=1.000000,G=0.000000,B=0.000000,A=1.000000)" "(R=0.000000,G=1.000000,B=0.000000,A=1.000000)" 3.0))
  (if (<= (Math|Vector|Distance(Vector) (Variables|Default|GetLooteableOrigin) (.Location (Collision|BreakHitResult _outhit))) 1.5e+02)
    _
    (else
      (Variables|Default|SetLooteableOrigin (+ (* (Math|Vector|VectorUp) 1.5e+02) (.Location (Collision|BreakHitResult _outhit))))))
  (Class|DropLooteablesComponent|DropLooteables (Variables|Default|GetDropLooteables) (Variables|Default|GetLooteableOrigin) (Variables|Diseño|GetisDropLightMana?))
  (Class|DestructibleComponent|ApplyRadiusDamage (Variables|Default|GetDestructible1) 1.0 (Transformation|GetActorLocation) (Variables|Default|Getradius) (Variables|Default|Getimpulse) true)
  (switch Utilities|FlowControl|Switch|SwitchonE_RespawnTypes (Variables|Diseño|GetrespawnType)
    (:NewEnumerator0
      (Class|RespawnManager|AddtoAlwaysRespawnList _respawnman _self)
      (Collision|SetCollisionEnabled (Variables|Default|GetBox) "NoCollision" :!label _label)
      (bind _returnvalue (Utilities|Time|SetTimerbyEvent (delegate Custom|Hide) (Variables|Default|GetTimeDisappear)))
      (Variables|Default|SetGoHiddenHandle _returnvalue)
      (Physics|SetSimulatePhysics (Variables|Default|GetDestructible1) false))
    (:NewEnumerator1
      (Class|RespawnManager|AddtoRespawnUntilCheckpointList _respawnman _self)
      (goto _label))
    (:NewEnumerator2
      (Actor|DestroyActor))))

(event Custom|TotalHide
  (Physics|SetSimulatePhysics (Variables|Default|GetDestructible1) false)
  (Rendering|SetActorHiddenInGame true))

(event Custom|StopTimeLine
  (bind _newtrack_0 (Timeline|Timeline_0 Stop)
    (:Update
      (Rendering|Material|SetScalarParameterValueonMaterials (Variables|Default|GetDestructible1) "Opacity" _newtrack_0))))

(event EventBeginPlay
  (bind _box (Variables|Default|GetBox))
  (Utilities|FlowControl|Sequence
    (:then_0
      (bind _asscyther_game_mode_base (Utilities|Casting|CastToScytherGameModeBase (Game|GetGameMode)))
      (Variables|Default|SetScytherGameMode _asscyther_game_mode_base)
      (if (Variables|Diseño|GethasCollision?)
        (Collision|SetCollisionResponsetoAllChannels _box "ECR_Block")
        (Collision|SetCollisionResponsetoChannel _box "ECC_Visibility" "ECR_Ignore")
        (else
          (Collision|SetCollisionObjectType (Variables|Default|GetBox) "ECC_WorldDynamic")
          (Collision|SetCollisionResponsetoAllChannels (Variables|Default|GetBox) "ECR_Overlap")))
      (if (Variables|Diseño|GetcanPlayerStepOn?)
        (Collision|SetCollisionObjectType (Variables|Default|GetBox) "ECC_WorldStatic")))
    (:then_1
      (Variables|Default|SetinitialTransform (Transformation|GetActorTransform)))))

(event EventRespawn
  (bind _health (Variables|Default|GetHealth))
  (bind _gotruehiddenhandle (Variables|Default|GetGoTrueHiddenHandle))
  (bind _gohiddenhandle (Variables|Default|GetGoHiddenHandle))
  (Components|Activation|Activate (Variables|Default|GetNiagara) true)
  (CallFunction|RespawnDestructible)
  (Class|HealthComponent|ChangeHealth _health (Variables|/Script/Scyther.HealthComponent|GetmaxHp _health) "HEALING" false)
  (CallFunction|StopTimeLine)
  (Transformation|SetActorTransform (Variables|Default|GetinitialTransform))
  (Rendering|SetActorHiddenInGame false)
  (Collision|SetActorEnableCollision true)
  (Collision|SetCollisionEnabled (Variables|Default|GetBox) "QueryAndPhysics")
  (Physics|SetSimulatePhysics (Variables|Default|GetDestructible1) false)
  (Rendering|Material|SetScalarParameterValueonMaterials (Variables|Default|GetDestructible1) "Opacity" 1.0)
  (if (Utilities|Time|IsValidTimerHandle _gohiddenhandle)
    (Utilities|Time|ClearandInvalidateTimerbyHandle _gohiddenhandle))
  (if (Utilities|Time|IsValidTimerHandle _gotruehiddenhandle)
    (Utilities|Time|ClearandInvalidateTimerbyHandle _gotruehiddenhandle)))

(fn ConstructionScript)

(fn DoHitSound
  (if (not (Variables|Audio|GetisPlayingSounds?))
    (Variables|Audio|SetisPlayingSounds? true)
    (bind _returnvalue (Class|FMODBlueprintStatics|PlayEventAttached "/Game/FMOD/Events/Player/Scyther/Hit.Hit" (Variables|Default|GetDestructible1) "None" "0, 0, 0" "KeepRelativeOffset"))
    (Class|FMODAudioComponent|SetParameter _returnvalue "HitsVariety" (Utilities|Select :Index (Variables|Diseño|GetColission%20Material) :NewEnumerator0 0.0 :NewEnumerator1 1.0 :NewEnumerator2 2.0 :NewEnumerator4 3.0 :NewEnumerator3 4.0 :NewEnumerator5 5.0 :NewEnumerator6 6.0))
    (Class|FMODAudioComponent|Play _returnvalue)
    (Class|FMODAudioComponent|Release _returnvalue)
    (Variables|Audio|SetisPlayingSounds? false)))

(fn DestroySound
  (if (not (Variables|Audio|GetisPlayingBreakingSounds))
    (Variables|Audio|SetisPlayingBreakingSounds true)
    (bind _returnvalue (Class|FMODBlueprintStatics|PlayEventAttached "/Game/FMOD/Events/Enviroment/SFX/SFX_Breaking_Things/BreakingThings.BreakingThings" (Variables|Default|GetDestructible1) "None" "0, 0, 0" "KeepRelativeOffset"))
    (Class|FMODAudioComponent|SetParameter _returnvalue "BreakingSounds" (Utilities|Select :Index (Variables|Diseño|GetDestroyMaterials) :NewEnumerator0 0.0 :NewEnumerator1 1.0 :NewEnumerator2 2.0 :NewEnumerator3 3.0))
    (Class|FMODAudioComponent|Play _returnvalue)
    (Class|FMODAudioComponent|Release _returnvalue)
    (Variables|Audio|SetisPlayingBreakingSounds false)))

(fn DoForceEffect
  (ForceFeedback|SpawnForceFeedbackatLocation "/Game/Blueprints/ForceFeedback/FFE_HitDestruible.FFE_HitDestruible" (Transformation|GetWorldLocation (Variables|Default|GetDestructible1)) "0, 0, 0" false 1.0 0.0 0))

(fn RespawnDestructible
  (bind _destructible1 (Variables|Default|GetDestructible1))
  (bind _returnvalue (Class|DestructibleComponent|GetDestructibleMesh _destructible1))
  (LocalVariables|SetNewLocalVar_0 _returnvalue)
  (Class|DestructibleComponent|SetDestructibleMesh _destructible1)
  (Class|DestructibleComponent|SetDestructibleMesh (Variables|Default|GetDestructible1) (LocalVariables|GetNewLocalVar_0))
  (return))