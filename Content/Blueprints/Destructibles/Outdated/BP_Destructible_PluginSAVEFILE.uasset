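; Destructible prop Blueprint, stored under Outdated, that breaks at zero health and can respawn always, until checkpoint, or never.
; Zero health registers it with the game mode's respawn manager or destroys it, disables its trigger, then after a delay hides the mesh and resets fracture by reassigning it.
; Respawn restores visibility, health and collision.
; Bound events play attached hit and break sounds, parameterized by material.
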(event ZerohealthEvent(healthComp)
  (params (damageType :type DamageModes%20Enum :default "DASHEABLE"))
  (bind _self self)
  (bind _as_bp_game_mode (Variables|Default|GetAs%20BP%20Game%20Mode))
  (bind _respawnman (Variables|/Script/Scyther.ScytherGameModeBase|GetrespawnMan _as_bp_game_mode))
  (Utilities|FlowControl|Sequence
    (:then_0
      (switch Utilities|FlowControl|Switch|SwitchonE_RespawnTypes (Variables|Default|GetrespawnType)
        (:NewEnumerator0
          (Class|RespawnManager|AddtoAlwaysRespawnList _respawnman _self))
        (:NewEnumerator1
          (Class|RespawnManager|AddtoRespawnUntilCheckpointList _respawnman _self))
        (:NewEnumerator2
          (Actor|DestroyActor))))
    (:then_1
      (Collision|SetCollisionEnabled (Variables|Default|GetTriggerComponent) "NoCollision"))
    (:then_2
      (Utilities|FlowControl|Delay 2.0)
      (Rendering|SetVisibility (Variables|Default|GetDestructibleComponent) false true)
      (CallFunction|RespawnDestructible))))

(event Custom|Evento%20Hit%20Sound
  (CallFunction|DoHitSound))

(event Custom|Evento%20Destroy%20Sound
  (CallFunction|DestroySound))

(event EventBeginPlay
  (EventDispatchers|BindEventtoDoHitSound (delegate Custom|Evento%20Hit%20Sound))
  (EventDispatchers|BindEventtoDestroySound (delegate Custom|Evento%20Destroy%20Sound))
  (bind _asbp_game_mode (Utilities|Casting|CastToBP_GameMode (Game|GetGameMode)))
  (Variables|Default|SetAs%20BP%20Game%20Mode _asbp_game_mode))

(event Collision|EventActorBeginOverlap
  (params (OtherActor :type Actor%20Object%20Reference)))

(event EventTick
  (params (DeltaSeconds :type Float%20%28single-precision%29)))

(event EventRespawn
  (bind _healthcomp (Variables|Default|GethealthComp))
  (Rendering|SetVisibility (Variables|Default|GetDestructibleComponent) true true)
  (Class|HealthComponent|ChangeHealth _healthcomp (Variables|/Script/Scyther.HealthComponent|GetmaxHp _healthcomp) "HEALING" true)
  (Collision|SetCollisionEnabled (Variables|Default|GetTriggerComponent) "QueryAndPhysics"))

(fn ConstructionScript)

(fn DoHitSound
  (bind _returnvalue (Class|FMODBlueprintStatics|PlayEventAttached "/Game/FMOD/Events/Player/Scyther/Hit.Hit" (Variables|Default|GetDestructibleComponent) "None" "0, 0, 0" "KeepRelativeOffset"))
  (Class|FMODAudioComponent|SetParameter _returnvalue "HitsVariety" (Utilities|Select :Index (Variables|Design|GetCollisionMaterial) :NewEnumerator0 0.0 :NewEnumerator1 1.0 :NewEnumerator2 2.0 :NewEnumerator4 3.0 :NewEnumerator3 4.0 :NewEnumerator5 0.0))
  (Class|FMODAudioComponent|Play _returnvalue)
  (Class|FMODAudioComponent|Release _returnvalue))

(fn DestroySound
  (bind _returnvalue (Class|FMODBlueprintStatics|PlayEventAttached "/Game/FMOD/Events/Enviroment/SFX_Breaking_Things/BreakingThings.BreakingThings" (Variables|Default|GetDestructibleComponent) "None" "0, 0, 0" "KeepRelativeOffset"))
  (Class|FMODAudioComponent|SetParameter _returnvalue "BreakingSounds" (Utilities|Select :Index (Variables|Design|GetDestroyMaterial) :NewEnumerator0 0.0 :NewEnumerator1 1.0 :NewEnumerator2 2.0 :NewEnumerator3 0.0))
  (Class|FMODAudioComponent|Play _returnvalue)
  (Class|FMODAudioComponent|Release _returnvalue))

(fn RespawnDestructible
  (bind _destructiblecomponent (Variables|Default|GetDestructibleComponent))
  (bind _returnvalue (Class|DestructibleComponent|GetDestructibleMesh _destructiblecomponent))
  (LocalVariables|SetNewLocalVar_0 _returnvalue)
  (Class|DestructibleComponent|SetDestructibleMesh _destructiblecomponent)
  (Class|DestructibleComponent|SetDestructibleMesh (Variables|Default|GetDestructibleComponent) (LocalVariables|GetNewLocalVar_0)))