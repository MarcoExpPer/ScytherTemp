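; Destructible platform that tilts when the player steps on it, breaks after a delay and later respawns.
; A PlayerBody overlap on Box1 rotates the destructible, plays a hit sound and starts the break timer, which destroys it and starts the respawn timer.
; Respawn clears the active flag and timers and restores the initial actor rotation.
; The GameMode's player respawn event also clears both timers and restores rotation, but leaves the active flag untouched.
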(event OnComponentBeginOverlap(Box1)
  (params (OverlappedComponent :type Primitive%20Component%20Object%20Reference) (OtherActor :type Actor%20Object%20Reference) (OtherComp :type Primitive%20Component%20Object%20Reference) (OtherBodyIndex :type Integer) (bFromSweep :type Boolean) (SweepResult :type Hit%20Result%20Structure%20%28by%20ref%29))
  (if (and (Components|ComponentHasTag OtherComp "PlayerBody") (not (Variables|Default|GetisActive?)))
    (Variables|Default|SetisActive? true)
    (bind _returnvalue (Utilities|Time|SetTimerbyEvent (delegate Custom|DestroyDes) (Variables|Default|GettimeToBreak)))
    (Variables|Default|SetBreakTimerHandle _returnvalue)
    (Transformation|AddWorldRotation (Variables|Default|GetDestructible1) (Variables|Default|GetRotationOffset) false false)
    (CallFunction|DoHitSound)))

(event Custom|DestroyDes
  (CallFunction|DestroyDestructible)
  (bind _returnvalue (Utilities|Time|SetTimerbyEvent (delegate Custom|RespawnPlatform) (Variables|Default|GettimeToRespawn)))
  (Variables|Default|SetRespawnTimerHandle _returnvalue))

(event Custom|StopTimer
  (params (location :type Vector))
  (Utilities|RemoveHandlesandRotation))

(event Custom|RespawnPlatform
  (Class|CanRespawn|Respawn))

(event EventBeginPlay
  (|CallParentFunction)
  (Utilities|FlowControl|Delay 0.2)
  (bind _asbp_game_mode (Utilities|Casting|CastToBP_GameMode (Game|GetGameMode)))
  (EventDispatchers|BindEventtoPlayerRespawnEvent (Variables|/Script/Scyther.ScytherGameModeBase|GetrespawnMan _asbp_game_mode) (delegate Custom|StopTimer))
  (Variables|Default|SetinitialRotation (Transformation|GetActorRotation)))

(event Collision|EventActorBeginOverlap
  (params (OtherActor :type Actor%20Object%20Reference)))

(event EventTick
  (params (DeltaSeconds :type Float%20%28single-precision%29)))

(event EventRespawn
  (|CallParentFunction)
  (Variables|Default|SetisActive? false)
  (Utilities|RemoveHandlesandRotation))

(fn ConstructionScript
  (|CallParentFunction))