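; BP_Destructible is a destructible prop with configurable physics and collision that drops lootables when broken.
; Health damage triggers material-specific FMOD-style hit audio and force feedback.
; At zero health, a destructible prop plays break audio, enables physics and fades via a delayed opacity loop, then drops loot.
; It then registers with the game mode's respawn manager or is destroyed, and Respawn restores health, transform, visibility and collision.
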(event HealthChangedEvent(Health)
  (params (oldHp :type Float%20%28single-precision%29) (newHp :type Float%20%28single-precision%29) (damageType :type DamageModes%20Enum :default "DASHEABLE"))
  (if (< newHp oldHp)
    (CallFunction|DoHitSound)
    (CallFunction|DoForceEffect)))

(event ZerohealthEvent(Health)
  (params (damageType :type DamageModes%20Enum :default "DASHEABLE"))
  (bind _self self)
  (bind _scythergamemode (Variables|Default|GetScytherGameMode))
  (bind _respawnman (Variables|/Script/Scyther.ScytherGameModeBase|GetrespawnMan _scythergamemode))
  (if (Variables|Diseño|GetIsDestruible)
    (CallFunction|DestroySound)
    (Variables|Default|SetLooteableOrigin (.Origin (Collision|GetActorBounds false false)))
    (Physics|SetSimulatePhysics (Variables|Default|GetDestructible) true)
    (Collision|SetActorEnableCollision false)
    ;[1 1 1] DisappearObject
    (Variables|Default|SetOpacity (- (Variables|Default|GetOpacity) (Variables|Default|GetDicreaseOpacity)) :!label _label)
    (Rendering|Material|SetScalarParameterValueonMaterials (Variables|Default|GetDestructible) "Opacity" (Variables|Default|GetOpacity))
    (if (<= (Variables|Default|GetOpacity) 0.0)
      (Class|DropLooteablesComponent|DropLooteables (Variables|Default|GetDropLooteables) (Variables|Default|GetLooteableOrigin) (Variables|Diseño|GetisDropLightMana?))
      (switch Utilities|FlowControl|Switch|SwitchonE_RespawnTypes (Variables|Diseño|GetrespawnType)
        (:NewEnumerator0
          (Class|RespawnManager|AddtoAlwaysRespawnList _respawnman _self)
          (Rendering|SetActorHiddenInGame true :!label _label_2)
          (Collision|SetActorEnableCollision false)
          (Physics|SetSimulatePhysics (Variables|Default|GetDestructible) false))
        (:NewEnumerator1
          (Class|RespawnManager|AddtoRespawnUntilCheckpointList _respawnman _self)
          (goto _label_2))
        (:NewEnumerator2
          (Actor|DestroyActor)))
      (else
        (Utilities|FlowControl|Delay (Variables|Default|GetTimeDisappear))
        (goto _label)))
    (else
      (CallFunction|DoHitSound))))

(event Custom|Initialize
  (Physics|SetSimulatePhysics (Variables|Default|GetDestructible) (Variables|Default|GethasPhysics))
  (if (Variables|Diseño|GethasCollision?)
    (Collision|SetCollisionResponsetoAllChannels (Variables|Default|GetBox) "ECR_Block")
    (if (Variables|Diseño|GetcanPlayerStepOn?)
      (Collision|SetCollisionObjectType (Variables|Default|GetBox) "ECC_WorldStatic"))
    (else
      (Collision|SetCollisionResponsetoAllChannels (Variables|Default|GetBox) "ECR_Overlap")
      (Collision|SetCollisionObjectType (Variables|Default|GetBox) "ECC_WorldDynamic"))))

(event EventBeginPlay
  (Utilities|FlowControl|Sequence
    (:then_0
      (bind _asscyther_game_mode_base (Utilities|Casting|CastToScytherGameModeBase (Game|GetGameMode)))
      (Variables|Default|SetScytherGameMode _asscyther_game_mode_base)
      (Physics|SetSimulatePhysics (Variables|Default|GetDestructible) (Variables|Default|GethasPhysics))
      (if (Variables|Diseño|GethasCollision?)
        (Collision|SetCollisionResponsetoAllChannels (Variables|Default|GetBox) "ECR_Block")
        (if (Variables|Diseño|GetcanPlayerStepOn?)
          (Collision|SetCollisionObjectType (Variables|Default|GetBox) "ECC_WorldStatic"))
        (else
          (Collision|SetCollisionResponsetoAllChannels (Variables|Default|GetBox) "ECR_Overlap")
          (Collision|SetCollisionObjectType (Variables|Default|GetBox) "ECC_WorldDynamic"))))
    (:then_1
      (Variables|Default|SetinitialTransform (Transformation|GetActorTransform)))
    (:then_2
      (Variables|Default|SethasPhysics (Physics|IsSimulatingPhysics (Variables|Default|GetDestructible) "None")))))

(event EventRespawn
  (bind _health (Variables|Default|GetHealth))
  (Class|HealthComponent|ChangeHealth _health (Variables|/Script/Scyther.HealthComponent|GetmaxHp _health) "HEALING" true)
  (Transformation|SetActorTransform (Variables|Default|GetinitialTransform))
  (Rendering|SetActorHiddenInGame false)
  (Collision|SetActorEnableCollision true))

(fn ConstructionScript)

(fn DoHitSound
  (if (not (Variables|Audio|GetisPlayingSounds?))
    (Variables|Audio|SetisPlayingSounds? true)
    (bind _returnvalue (Class|FMODBlueprintStatics|PlayEventAttached "/Game/FMOD/Events/Player/Scyther/Hit.Hit" (Variables|Default|GetDestructible) "None" "0, 0, 0" "KeepRelativeOffset"))
    (Utilities|IsValid _returnvalue
      (:Is%20Valid
        (Class|FMODAudioComponent|SetParameter _returnvalue "HitsVariety" (Utilities|Select :Index (Variables|Diseño|GetColission%20Material) :NewEnumerator0 0.0 :NewEnumerator1 1.0 :NewEnumerator2 2.0 :NewEnumerator4 3.0 :NewEnumerator3 4.0 :NewEnumerator5 5.0 :NewEnumerator6 0.0))
        (Class|FMODAudioComponent|Play _returnvalue)
        (Class|FMODAudioComponent|Release _returnvalue)
        (Variables|Audio|SetisPlayingSounds? false)))))

(fn DestroySound
  (if (not (Variables|Audio|GetisPlayingBreakingSounds?))
    (Variables|Audio|SetisPlayingBreakingSounds? true)
    (bind _returnvalue (Class|FMODBlueprintStatics|PlayEventAttached "/Game/FMOD/Events/Enviroment/SFX_Breaking_Things/BreakingThings.BreakingThings" (Variables|Default|GetDestructible) "None" "0, 0, 0" "KeepRelativeOffset"))
    (Utilities|IsValid _returnvalue
      (:Is%20Valid
        (Class|FMODAudioComponent|SetParameter _returnvalue "BreakingSounds" (Utilities|Select :Index (Variables|Diseño|GetDestroyMaterials) :NewEnumerator0 0.0 :NewEnumerator1 1.0 :NewEnumerator2 2.0 :NewEnumerator3 3.0))
        (Class|FMODAudioComponent|Play _returnvalue)
        (Class|FMODAudioComponent|Release _returnvalue))
      (:Is%20Not%20Valid
        _))
    (Variables|Audio|SetisPlayingBreakingSounds? false)))

(fn DoForceEffect
  (ForceFeedback|SpawnForceFeedbackatLocation "/Game/Blueprints/ForceFeedback/FFE_HitDestruible.FFE_HitDestruible" (Transformation|GetWorldLocation (Variables|Default|GetDestructible)) "0, 0, 0" false 1.0 0.0 0))