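; Side-scrolling camera actor that tracks a target actor, with its X position held fixed.
; Each tick it aims the camera component at the target and maps the target's distance to a clamped alpha between min and max range.
; That alpha blends near and far values for both an interpolated FOV and a vertical offset.
; The actor eases in Y and Z toward the midpoint between itself and the target, plus that offset.
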(event EventBeginPlay)

(event EventTick
  (params (DeltaSeconds :type Float%20%28single-precision%29))
  (bind _returnvalue (Transformation|GetActorLocation))
  (bind _cameracomponent (Variables|CameraActor|GetCameraComponent))
  (bind _targetactor (Variables|SideScroller|GetTargetActor))
  (bind _returnvalue_2 (Transformation|GetActorLocation _targetactor))
  (bind _returnvalue_3 (Math|Vector|Lerp(Vector) _returnvalue_2 _returnvalue 0.5))
  (Utilities|IsValid (Variables|SideScroller|GetTargetActor)
    (:Is%20Valid
      ;[1 1 1] Camera looks to player
      (Transformation|SetWorldRotation (Variables|CameraActor|GetCameraComponent) (Math|Rotator|FindLookatRotation (Transformation|GetActorLocation) (Transformation|GetActorLocation (Variables|SideScroller|GetTargetActor))) false false)
      ;[1 1 1] Update camera field of view
      (Variables|Default|SetTargetDistance (Transformation|GetDistanceTo (Variables|SideScroller|GetTargetActor)))
      (Variables|Default|SetCurrentDistanceAlpha (Math|Float|Clamp(Float) (Math|Float|NormalizetoRange (Variables|Default|GetTargetDistance) (Variables|SideScroller|GetMinDistance) (Variables|SideScroller|GetMaxDistance))))
      (Camera|SetFieldOfView _cameracomponent (Math|Interpolation|FInterpTo (Variables|/Script/Engine.CameraComponent|GetFieldOfView _cameracomponent) (Math|Float|Lerp (Variables|SideScroller|GetNearFOV) (Variables|SideScroller|GetFarFOV) (Variables|Default|GetCurrentDistanceAlpha)) (Utilities|Time|GetWorldDeltaSeconds) (Variables|SideScroller|GetFOVSpeed)))
      (Transformation|SetActorLocation (Math|Interpolation|VInterpTo _returnvalue (Math|Vector|MakeVector (.X (Math|Vector|BreakVector _returnvalue)) (.y _returnvalue_3) (+ (.z _returnvalue_3) (Math|Float|Lerp (Variables|SideScroller|GetNearVerticalOffset) (Variables|SideScroller|GetFarVerticalOffset) (Variables|Default|GetCurrentDistanceAlpha)))) (Utilities|Time|GetWorldDeltaSeconds) (Variables|Default|GetCameraSpeed)) false false))))

(fn ConstructionScript)