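; BP_TimerDoT is a component that applies damage over time to the actor it is attached to.
; On BeginPlay it caches the owner's HealthComponent, or destroys itself if none exists.
; Tick counts down the duration and interval timers, sending INEVITABLE damage immediately and then whenever the interval elapses.
; It destroys itself once the duration runs out or the HealthComponent becomes invalid.
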(event EventBeginPlay
  (bind _returnvalue (Components|GetOwner))
  (bind _returnvalue_2 (Actor|GetComponentbyClass _returnvalue "/Script/Scyther.HealthComponent"))
  (Utilities|IsValid _returnvalue_2
    (:Is%20Valid
      (Variables|Default|SetHealthComponent _returnvalue_2)
      (Variables|Daño|SettiempoHastaElTick 0.0))
    (:Is%20Not%20Valid
      ;[1 1 1] Si el objetivo no es dañable, destruimos este componente
      (Components|DestroyComponent))))

(event EventTick
  (params (DeltaSeconds :type Float%20%28single-precision%29))
  ;[1 1 1] Comprobar si el objetivo esta muerto
  (if (Utilities|IsValid (Variables|Default|GetHealthComponent))
    ;[1 1 1] Comprobar si el efecto ya ha ocurrido por completo
    (if (<= (Variables|Daño|GetDoTDuration) 0.0)
      (Components|DestroyComponent)
      (else
        ;[1 1 1] Comprobar si hay que hacer el daño
        (if (<= (Variables|Daño|GettiempoHastaElTick) 0.0)
          ;[1 1 1] Realizar el daño
          (Variables|Daño|SettiempoHastaElTick (Variables|Daño|GettickTimer))
          (Class|HealthComponent|ReceiveDamage (Variables|Default|GetHealthComponent) (Variables|Daño|GetdamagePerTick) "INEVITABLE" true)
          (else
            ;[1 1 1] Reducir los timers
            (Variables|Daño|SetDoTDuration (- (Variables|Daño|GetDoTDuration) (Utilities|Time|GetWorldDeltaSeconds)))
            (Variables|Daño|SettiempoHastaElTick (- (Variables|Daño|GettiempoHastaElTick) (Utilities|Time|GetWorldDeltaSeconds)))))))
    (else
      (Components|DestroyComponent))))