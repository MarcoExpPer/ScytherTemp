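; BP_ManualDoT is a damage-over-time Blueprint that periodically hurts registered actors with DEADZONE damage through their HealthComponent.
; AddActor registers actors that have a HealthComponent with a zero timer, and RemoveActor unregisters them.
; Tick counts each timer down, applying DamagePerTick and resetting to TickTimer on expiry.
; Timers are keyed by array index rather than actor, so removals can misalign them.
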(event Custom|AddActor
  (params (Actor :type Actor%20Object%20Reference))
  ;[1 1 1] Añade el actor a la lista de actores que van a recibir daño, e inicializa su timer
  (Utilities|IsValid (Actor|GetComponentbyClass Actor "/Script/Scyther.HealthComponent")
    (:Is%20Valid
      (bind _returnvalue (Utilities|Array|AddUnique (Variables|Default|GetAffectedActors) Actor))
      (Utilities|Map|Add (Variables|Default|GetActorToTickTimer) _returnvalue 0.0))))

(event Custom|RemoveActor
  (params (Actor :type Actor%20Object%20Reference))
  (bind _affectedactors (Variables|Default|GetAffectedActors))
  (bind _returnvalue (Utilities|Array|FindItem _affectedactors Actor))
  ;[1 1 1] Elimina un actor de la lista
  (Utilities|Map|Remove (Variables|Default|GetActorToTickTimer) _returnvalue)
  (Utilities|Array|RemoveIndex (Variables|Default|GetAffectedActors) _returnvalue))

(event EventTick
  (params (DeltaSeconds :type Float%20%28single-precision%29))
  ;[1 1 1] Daña a todos los actores que les toque y avanza los timers de los que no
  (for (_array_element _array_index) (Variables|Default|GetAffectedActors)
    (if (and (<= (.Value (Utilities|Map|Find (Variables|Default|GetActorToTickTimer) _array_index)) 0.0) (.ReturnValue (Utilities|Map|Find (Variables|Default|GetActorToTickTimer) _array_index)))
      (Utilities|Map|Add (Variables|Default|GetActorToTickTimer) _array_index (Variables|Daño|GettickTimer))
      (Utilities|IsValid (Actor|GetComponentbyClass _array_element "/Script/Scyther.HealthComponent")
        (:Is%20Valid
          (Class|HealthComponent|ReceiveDamage (Actor|GetComponentbyClass _array_element "/Script/Scyther.HealthComponent") (Variables|Daño|GetdamagePerTick) "DEADZONE" true)))
      (else
        (Utilities|Map|Add (Variables|Default|GetActorToTickTimer) _array_index (- (.Value (Utilities|Map|Find (Variables|Default|GetActorToTickTimer) _array_index)) (Utilities|Time|GetWorldDeltaSeconds)))))))