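; AI controller for the old version of the rabbit enemy, running its behavior tree.
; After a short delay on BeginPlay, it sets up the blackboard, seeds it with the pawn's light mode, spawn-time location as home, and attack and detection distances, then starts the tree.
; The rabbit pawn's TurnDark and TurnLight events update the IsLightMode key so the tree tracks the current mode.
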(event TurnDarkEvent(rabbitPawn)
  (AI|Components|Blackboard|SetValueasBool (Variables|Default|GetBlackboard%20Component) (Variables|BlackBoardNames|GetisLightMode?) false))

(event TurnLightEvent(rabbitPawn)
  (AI|Components|Blackboard|SetValueasBool (Variables|Default|GetBlackboard%20Component) (Variables|BlackBoardNames|GetisLightMode?) true))

(event EventBeginPlay
  (|CallParentFunction)
  (Utilities|FlowControl|Delay 0.2)
  (bind _blackboardcomponent (Class|AIController|UseBlackboard "/Game/Blueprints/Enemies/Conejo/OLD/BB_OldRabbit.BB_OldRabbit"))
  (Variables|Default|SetBlackboard%20Component _blackboardcomponent)
  (CallFunction|InitBBValues)
  (AI|RunBehaviorTree "/Game/Blueprints/Enemies/Conejo/OLD/BTT_OldRabbit.BTT_OldRabbit"))

(fn ConstructionScript)

(fn InitBBValues
  (AI|Components|Blackboard|SetValueasBool (Variables|Default|GetBlackboard%20Component) (Variables|BlackBoardNames|GetisLightMode?) (Variables|/Script/Scyther.BaseEnemy|GetisLightMode (Variables|Default|GetrabbitPawn)))
  (AI|Components|Blackboard|SetValueasFloat (Variables|Default|GetBlackboard%20Component) (Variables|BlackBoardNames|GetminimumDistanceToAttackName) (Variables|Default|GetdistanceToAttackPlayer))
  (AI|Components|Blackboard|SetValueasVector (Variables|Default|GetBlackboard%20Component) (Variables|BlackBoardNames|GethomeLocationname) (Transformation|GetActorLocation (Variables|Default|GetrabbitPawn)))
  (AI|Components|Blackboard|SetValueasFloat (Variables|Default|GetBlackboard%20Component) (Variables|BlackBoardNames|GetdistanceToDetectPlayerName) (Variables|Default|GetdistanceToDetectPlayer)))