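; Older rabbit enemy Blueprint that changes its look with the game's light/dark state.
; Body and cone materials are set from IsLightMode at construction and whenever a turn-dark or turn-light event fires.
; Health loss plays a timeline that drives the AlphaDamage material parameter on the body as a hit effect.
; Cone overlaps and hits with components tagged PlayerBody only print a debug string.
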(event HealthChangedEvent(healthComp)
  (params (oldHp :type Float%20%28single-precision%29) (newHp :type Float%20%28single-precision%29) (damageType :type DamageModes%20Enum :default "DASHEABLE"))
  (if (< newHp oldHp)
    ;[1 1 1] VFX_Damage
    (bind _time_damage (Timeline|Timeline_Damage PlayFromStart)
      (:Update
        (Rendering|Material|SetScalarParameterValueonMaterials (Variables|Default|GetrabbitBody) "AlphaDamage" _time_damage)))))

(event OnComponentBeginOverlap(Cone)
  (params (OverlappedComponent :type Primitive%20Component%20Object%20Reference) (OtherActor :type Actor%20Object%20Reference) (OtherComp :type Primitive%20Component%20Object%20Reference) (OtherBodyIndex :type Integer) (bFromSweep :type Boolean) (SweepResult :type Hit%20Result%20Structure%20%28by%20ref%29))
  (if (Components|ComponentHasTag OtherComp "PlayerBody")
    (Development|PrintString "Hello")))

(event OnComponentHit(Cone)
  (params (HitComponent :type Primitive%20Component%20Object%20Reference) (OtherActor :type Actor%20Object%20Reference) (OtherComp :type Primitive%20Component%20Object%20Reference) (NormalImpulse :type Vector :default "0, 0, 0") (Hit :type Hit%20Result%20Structure%20%28by%20ref%29))
  (if (Components|ComponentHasTag OtherComp "PlayerBody")
    (Development|PrintString "Hello")))

(event Custom|ChangeBalanceEvent
  (Utilities|ChangeTextureBasedonLight))

(event EventBeginPlay
  (|CallParentFunction)
  (EventDispatchers|AssignTurnDarkEvent (delegate Custom|ChangeBalanceEvent))
  (EventDispatchers|AssignTurnLightEvent (delegate Custom|ChangeBalanceEvent)))

(event Collision|EventActorBeginOverlap
  (params (OtherActor :type Actor%20Object%20Reference)))

(event EventTick
  (params (DeltaSeconds :type Float%20%28single-precision%29)))

(fn ConstructionScript
  (Utilities|ChangeTextureBasedonLight))