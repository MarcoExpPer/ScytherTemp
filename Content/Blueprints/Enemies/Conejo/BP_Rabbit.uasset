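; BP_Rabbit is a rabbit enemy that switches between light and dark looks and displays its health as debug text.
; A HealthComp change event refreshes the text, which is also initialized on BeginPlay.
; The TurnDark and TurnLight events share one handler that swaps body and cone materials according to IsLightMode.
; The construction script runs the same material swap, so the look matches the mode at construction.
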(event Custom|healthChangedEvent_Event_0
  (params (oldHp :type Float%20%28single-precision%29) (newHp :type Float%20%28single-precision%29) (damageType :type ElementTypes%20Enum :default "NEUTRAL"))
  ;[1 1 1] Change Debug health text when hit
  (Rendering|Components|TextRender|SetText (Variables|Default|Gethealth) (Utilities|Text|ToText(Float) newHp "HalfToEven")))

(event Custom|turnDarkEvent_Event_0
  (Utilities|ChangeTextureBasedonLight))

(event EventBeginPlay
  (|CallParentFunction)
  ;[1 1 1] Change Debug health text when hit
  (EventDispatchers|AssignHealthChangedEvent (Variables|Default|GethealthComp) (delegate Custom|healthChangedEvent_Event_0))
  (Rendering|Components|TextRender|SetText (Variables|Default|Gethealth) (Utilities|Text|ToText(Float) (Variables|/Script/Scyther.HealthComponent|GetcurrentHp (Variables|Default|GethealthComp)) "HalfToEven"))
  (EventDispatchers|AssignTurnDarkEvent (delegate Custom|turnDarkEvent_Event_0))
  (EventDispatchers|AssignTurnLightEvent (delegate Custom|turnDarkEvent_Event_0)))

(event Collision|EventActorBeginOverlap
  (params (OtherActor :type Actor%20Object%20Reference)))

(event EventTick
  (params (DeltaSeconds :type Float%20%28single-precision%29)))

(fn ConstructionScript
  (Utilities|ChangeTextureBasedonLight))