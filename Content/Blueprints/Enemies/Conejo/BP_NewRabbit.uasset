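; Rabbit enemy that reacts to the light/dark mode, swapping its skeleton material and whether its box collision blocks the Visibility channel.
; A timeline fades the material during the turn to dark, and a Niagara effect fires on the change.
; Damage plays a material-based hit sound and cycles three splat meshes as timed VFX; immune hits play only sound.
; Tick locks spawn height, and hat overlaps with an airborne player nudge the rabbit.
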(event HealthChangedEvent(healthComp)
  (params (oldHp :type Float%20%28single-precision%29) (newHp :type Float%20%28single-precision%29) (damageType :type DamageModes%20Enum :default "DASHEABLE"))
  (bind _spla1 (Variables|Default|Getspla1))
  (bind _splat2 (Variables|Default|Getsplat2))
  (bind _splat3 (Variables|Default|Getsplat3))
  (bind _vfxindex (Variables|Default|GetvfxIndex))
  (bind _returnvalue (Utilities|Select :Index _vfxindex :Option%200 _spla1 :Option%201 _splat2 :Option%202 _splat3))
  (if (< newHp oldHp)
    (Utilities|FlowControl|Sequence
      (:then_0
        (bind _returnvalue_2 (Class|FMODBlueprintStatics|PlayEventAttached "/Game/FMOD/Events/Player/Scyther/Hit.Hit" (Variables|Default|GetrabbitBoxColisionS) "None" "0, 0, 0" "KeepRelativeOffset"))
        (Class|FMODAudioComponent|SetParameter _returnvalue_2 "HitsVariety" (Utilities|Select :Index (Variables|Default|GetColission%20Material) :NewEnumerator0 0.0 :NewEnumerator1 1.0 :NewEnumerator2 2.0 :NewEnumerator4 3.0 :NewEnumerator3 4.0 :NewEnumerator5 5.0 :NewEnumerator6 0.0))
        (Class|FMODAudioComponent|Play _returnvalue_2)
        (Class|FMODAudioComponent|Release _returnvalue_2))
      (:then_1
        (CallFunction|MoveVFX)
        (Utilities|Time|ClearandInvalidateTimerbyHandle (Variables|Default|GetNewVar_0))
        (Rendering|Material|SetMaterial _returnvalue 0 0)
        (Rendering|Material|SetScalarParameterValueonMaterials _returnvalue "Game Time At First Frame" (Utilities|Time|GetTimeSeconds))
        (Rendering|SetVisibility _returnvalue true false)
        (CallFunction|HideVFXHit (Variables|Default|GetvfxIndex))
        (Utilities|UpdateVFX)))))

(event InmuneHitEvent(healthComp)
  (params (damageType :type DamageModes%20Enum :default "DASHEABLE"))
  (bind _returnvalue (Class|FMODBlueprintStatics|PlayEventAttached "/Game/FMOD/Events/Player/Scyther/Hit.Hit" (Variables|Default|GetrabbitBoxColisionS) "None" "0, 0, 0" "KeepRelativeOffset"))
  (Class|FMODAudioComponent|SetParameter _returnvalue "HitsVariety" 1.0)
  (Class|FMODAudioComponent|Play _returnvalue)
  (Class|FMODAudioComponent|Release _returnvalue))

(event OnComponentBeginOverlap(HatKnockback)
  (params (OverlappedComponent :type Primitive%20Component%20Object%20Reference) (OtherActor :type Actor%20Object%20Reference) (OtherComp :type Primitive%20Component%20Object%20Reference) (OtherBodyIndex :type Integer) (bFromSweep :type Boolean) (SweepResult :type Hit%20Result%20Structure%20%28by%20ref%29))
  (bind (_bblockinghit _binitialoverlap _time _distance _location _impactpoint _normal _impactnormal _physmat _hitactor _hitcomponent _hitbonename _hititem _elementindex _faceindex _tracestart _traceend) (Collision|BreakHitResult SweepResult))
  (bind _returnvalue (- _traceend _tracestart))
  (bind _returnvalue_2 (Math|Vector|Normalize _returnvalue))
  (bind _returnvalue_3 (* _returnvalue_2 1e+01))
  (if (Components|ComponentHasTag OtherComp "PlayerBody")
    (bind _asbp_scyther_player_pawn (Utilities|Casting|CastToBP_ScytherPlayerPawn OtherActor))
    (if (or (Utilities|Enum|Equal(Enum) (Variables|/Script/Scyther.ScytherPlayerPawn|Getstate _asbp_scyther_player_pawn) "INAPEX") (Utilities|Enum|Equal(Enum) (Variables|/Script/Scyther.ScytherPlayerPawn|Getstate _asbp_scyther_player_pawn) "FALLING"))
      (Transformation|AddActorWorldOffset (Math|Vector|MakeVector (.x _returnvalue_3) (.y _returnvalue_3) 0.0)))))

(event Custom|isLightMdoeChanged
  (bind _rabbitboxcolisions (Variables|Default|GetrabbitBoxColisionS))
  (Utilities|ChangeTextureBasedonLightMode
    (:Exit
      (if (Variables|Default|GetisLightMode)
        (Collision|SetCollisionResponsetoChannel _rabbitboxcolisions "ECC_Visibility" "ECR_Ignore")
        (else
          (Collision|SetCollisionResponsetoChannel _rabbitboxcolisions "ECC_Visibility" "ECR_Block"))))))

(event Custom|turningDarkEvent_Event_0
  (params (timeToTurn :type Float%20%28single-precision%29))
  (Utilities|FlowControl|Sequence
    (:then_0
      (bind _newtrack_0 (Timeline|Timeline_1 PlayFromStart)
        (:Update
          ;[1 1 1] VFX_TurningDark
          (Rendering|Material|SetScalarParameterValueonMaterials (Variables|Default|GetrabbitSkeleton) "AlphaChangeToDark" _newtrack_0))))
    (:then_1
      (Timeline|Timeline_1 SetNewTime))))

(event Custom|HideVFXHit
  (params (index :type Integer))
  (bind _splat3 (Variables|Default|Getsplat3))
  (bind _spla1 (Variables|Default|Getspla1))
  (bind _splat2 (Variables|Default|Getsplat2))
  (switch int index
    (:Default
      (Utilities|FlowControl|Delay 1.0 :!label _label)
      (Rendering|SetVisibility _splat3 false false)
      (Rendering|Material|SetMaterial _splat3 0 0))
    (:0
      (Utilities|FlowControl|Delay 1.0)
      (Rendering|SetVisibility _spla1 false false)
      (Rendering|Material|SetMaterial _spla1 0 0))
    (:1
      (Utilities|FlowControl|Delay 1.0)
      (Rendering|SetVisibility _splat2 false false)
      (Rendering|Material|SetMaterial _splat2 0 0))
    (:2
      (goto _label))))

(event Custom|PlayChangeVFX
  (Components|Activation|Activate (Variables|Default|GetNiagara) false))

(event EventBeginPlay
  (|CallParentFunction)
  (EventDispatchers|AssignTurnDarkEvent (delegate Custom|isLightMdoeChanged))
  (EventDispatchers|AssignTurnLightEvent (delegate Custom|isLightMdoeChanged))
  (Variables|Default|SetvfxIndex 0)
  (EventDispatchers|AssignTurningDarkEvent (delegate Custom|turningDarkEvent_Event_0))
  (EventDispatchers|BindEventtoTurnDarkEvent (delegate Custom|PlayChangeVFX)))

(event EventTick
  (params (DeltaSeconds :type Float%20%28single-precision%29))
  (bind _returnvalue (Transformation|GetActorLocation))
  (Transformation|SetActorLocation (Math|Vector|MakeVector (.x _returnvalue) (.y _returnvalue) (.z (.location (Variables|Default|GetinitialTransform)))) false false))

(fn ConstructionScript
  (bind _spla1 (Variables|Default|Getspla1))
  (bind _rabbitboxcolisions (Variables|Default|GetrabbitBoxColisionS))
  (Utilities|ChangeTextureBasedonLightMode
    (:Exit
      (CallFunction|MoveVFX)
      (Variables|Default|SetVAT_Mat (Rendering|Material|GetMaterial _spla1 0))
      (Rendering|Material|SetMaterial _spla1 0 0)
      (Transformation|SetWorldTransform (Variables|Default|Getsplat2) (Transformation|GetWorldTransform (Variables|Default|Getspla1)) true true)
      (if (Variables|Default|GetisLightMode)
        (Collision|SetCollisionResponsetoChannel _rabbitboxcolisions "ECC_Visibility" "ECR_Ignore")
        (else
          (Collision|SetCollisionResponsetoChannel _rabbitboxcolisions "ECC_Visibility" "ECR_Block"))))))

(fn MoveVFX
  (bind _returnvalue (Transformation|GetActorLocation))
  (bind _returnvalue_2 (Transformation|GetActorForwardVector))
  (bind _hitvfxoffset (Variables|Default|GethitVFXOffset))
  (bind _returnvalue_3 (* _returnvalue_2 (.x _hitvfxoffset)))
  (bind _returnvalue_4 (+ _returnvalue_3 _returnvalue))
  (Transformation|SetWorldLocation (Utilities|Select :Index (Variables|Default|GetvfxIndex) :Option%200 (Variables|Default|Getspla1) :Option%201 (Variables|Default|Getsplat2) :Option%202 (Variables|Default|Getsplat3)) (Math|Vector|MakeVector (.x _returnvalue_4) (.y _returnvalue_4) (+ (.z (Transformation|GetActorLocation)) (.z _hitvfxoffset))) false true)
  (return))