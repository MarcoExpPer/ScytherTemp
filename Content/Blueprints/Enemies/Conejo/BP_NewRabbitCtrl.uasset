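; AI controller for the rabbit enemy BP_NewRabbit that sets up its blackboard and starts its behavior tree.
; After a short delay on BeginPlay, it caches the controlled pawn and copies its attack, detection and return-home distances, plus home location, into BB_NewRabbit.
; If the pawn's GoToLocation flag is set, it also seeds the move destination.
; It then runs BTT_NewRabbit and passes that flag to the pawn's ToggleAI.
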(event EventBeginPlay
  (Utilities|FlowControl|Delay 0.2)
  (bind _asbp_new_rabbit (Utilities|Casting|CastToBP_NewRabbit (Pawn|GetControlledPawn)))
  (Variables|Default|SetnewRabbitPawnBP _asbp_new_rabbit)
  (bind _blackboardcomponent (Class|AIController|UseBlackboard "/Game/Blueprints/Enemies/Conejo/BB_NewRabbit.BB_NewRabbit"))
  (Variables|Default|SetBlackboard%20Component _blackboardcomponent)
  (AI|Components|Blackboard|SetValueasFloat (Variables|Default|GetBlackboard%20Component) (Variables|BB|GetdistanceToAttackPlayerName) (Variables|/Game/Blueprints/Enemies/Conejo/BP_NewRabbit.BP_NewRabbit_C|GetDistanceToAttackPlayer (Variables|Default|GetnewRabbitPawnBP)))
  (AI|Components|Blackboard|SetValueasFloat (Variables|Default|GetBlackboard%20Component) (Variables|BB|GetdistanceToDetectPlayerName) (Variables|/Game/Blueprints/Enemies/Conejo/BP_NewRabbit.BP_NewRabbit_C|GetDistanceToDetectPlayer (Variables|Default|GetnewRabbitPawnBP)))
  (AI|Components|Blackboard|SetValueasFloat (Variables|Default|GetBlackboard%20Component) (Variables|BB|GetdistanceToReturnToHomeName) (Variables|/Game/Blueprints/Enemies/Conejo/BP_NewRabbit.BP_NewRabbit_C|GetDistanceToReturnToHome (Variables|Default|GetnewRabbitPawnBP)))
  (AI|Components|Blackboard|SetValueasVector (Variables|Default|GetBlackboard%20Component) (Variables|BB|GethomeLocationName) (.location (Variables|/Script/Scyther.BaseEnemy|GetinitialTransform (Variables|Default|GetnewRabbitPawnBP))))
  (Utilities|FlowControl|Sequence
    (:then_0
      (if (Variables|/Game/Blueprints/Enemies/Conejo/BP_NewRabbit.BP_NewRabbit_C|GetGoToLocation? (Variables|Default|GetnewRabbitPawnBP))
        (Class|NewRabbitPawnBase|SetNewTarget (Variables|Default|GetnewRabbitPawnBP) "GoToLocation")
        (AI|Components|Blackboard|SetValueasVector (Variables|Default|GetBlackboard%20Component) (Variables|BB|GetLocationToMoveToName) (Variables|/Game/Blueprints/Enemies/Conejo/BP_NewRabbit.BP_NewRabbit_C|GetLocationToMoveTo (Variables|Default|GetnewRabbitPawnBP)))))
    (:then_1
      (AI|RunBehaviorTree "/Game/Blueprints/Enemies/Conejo/BTT_NewRabbit.BTT_NewRabbit")
      (Class|BaseEnemy|ToggleAI (Variables|Default|GetnewRabbitPawnBP) (Variables|/Game/Blueprints/Enemies/Conejo/BP_NewRabbit.BP_NewRabbit_C|GetGoToLocation? (Variables|Default|GetnewRabbitPawnBP))))))

(fn ConstructionScript)