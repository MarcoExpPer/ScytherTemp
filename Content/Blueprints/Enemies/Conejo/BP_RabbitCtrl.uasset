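; BP_RabbitCtrl is the AI controller for the Rabbit enemy.
; Shortly after BeginPlay it casts its pawn to BP_Rabbit, seeds BB_Rabbit with light mode, home location and attack and detection distances, then runs BTT_Rabbit.
; It binds to the rabbit's turn-dark and turn-light events to keep the blackboard's IsLightMode in sync for the behavior tree.
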(event Custom|turnDarkEvent_Event_0
  ;[1 1 1] Bind on balance mode change events, to tell the bb and the btt the mode changed
  (AI|Components|Blackboard|SetValueasBool (Variables|Default|GetBlackboard%20Component) (Variables|BlackBoardNames|GetisLightMode?) false))

(event Custom|turnLightEvent_Event_0
  ;[1 1 1] Bind on balance mode change events, to tell the bb and the btt the mode changed
  (AI|Components|Blackboard|SetValueasBool (Variables|Default|GetBlackboard%20Component) (Variables|BlackBoardNames|GetisLightMode?) true))

(event EventBeginPlay
  (|CallParentFunction)
  (Utilities|FlowControl|Delay 0.2)
  (bind _asbp_rabbit (Utilities|Casting|CastToBP_Rabbit (Pawn|GetControlledPawn)))
  (bind _output_get (Variables|Default|SetrabbitPawn _asbp_rabbit))
  ;[1 1 1] Bind on balance mode change events, to tell the bb and the btt the mode changed
  (EventDispatchers|AssignTurnDarkEvent _output_get (delegate Custom|turnDarkEvent_Event_0))
  (EventDispatchers|AssignTurnLightEvent _output_get (delegate Custom|turnLightEvent_Event_0))
  (bind _blackboardcomponent (Class|AIController|UseBlackboard "/Game/Blueprints/Enemies/Conejo/BB_Rabbit.BB_Rabbit"))
  (Variables|Default|SetBlackboard%20Component _blackboardcomponent)
  ;[1 1 1] Init bb light mode value
  (AI|Components|Blackboard|SetValueasBool (Variables|Default|GetBlackboard%20Component) (Variables|BlackBoardNames|GetisLightMode?) (Variables|/Script/Scyther.BaseEnemy|GetisLightMode (Variables|Default|GetrabbitPawn)))
  (AI|Components|Blackboard|SetValueasFloat (Variables|Default|GetBlackboard%20Component) (Variables|BlackBoardNames|GetminimumDistanceToAttackName) (Variables|Default|GetdistanceToAttackPlayer))
  (AI|Components|Blackboard|SetValueasVector (Variables|Default|GetBlackboard%20Component) (Variables|BlackBoardNames|GethomeLocationname) (Transformation|GetActorLocation (Variables|Default|GetrabbitPawn)))
  (AI|Components|Blackboard|SetValueasFloat (Variables|Default|GetBlackboard%20Component) (Variables|BlackBoardNames|GetdistanceToDetectPlayerName) (Variables|Default|GetdistanceToDetectPlayer))
  (AI|RunBehaviorTree "/Game/Blueprints/Enemies/Conejo/BTT_Rabbit.BTT_Rabbit"))

(fn ConstructionScript)