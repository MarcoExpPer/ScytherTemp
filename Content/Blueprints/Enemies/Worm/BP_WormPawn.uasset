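; Worm enemy pawn that switches its body between light and dark materials.
; The construction script picks the starting material from IsLightMode.
; BeginPlay binds the TurnDark and TurnLight events, which swap the WormBodyReal material at runtime.
; HorizontalAttack and Tick are empty, and a rotate-and-impulse lunge attack and a health debug print are left disconnected.
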(event Custom|Horizontal%20Attack)

(event Custom|turnDarkEvent_Event_0
  (Rendering|Material|SetMaterial (Variables|Default|GetwormBodyReal) 0 "/Game/Arte/Escena1/Enemies/Generic/Materials/M_Dark.M_Dark"))

(event Custom|turnLightEvent_Event_0
  (Rendering|Material|SetMaterial (Variables|Default|GetwormBodyReal) 0 "/Game/Arte/Escena1/Enemies/Generic/Materials/M_Light.M_Light"))

(event EventBeginPlay
  (EventDispatchers|AssignTurnDarkEvent (delegate Custom|turnDarkEvent_Event_0))
  (EventDispatchers|AssignTurnLightEvent (delegate Custom|turnLightEvent_Event_0)))

(event EventTick
  (params (DeltaSeconds :type Float%20%28single-precision%29)))

(fn ConstructionScript
  (if (Variables|Default|GetisLightMode)
    (Rendering|Material|SetMaterial (Variables|Default|GetwormBodyReal) 0 "/Game/Arte/Escena1/Enemies/Generic/Materials/M_Light.M_Light")
    (else
      (Rendering|Material|SetMaterial (Variables|Default|GetwormBodyReal) 0 "/Game/Arte/Escena1/Enemies/Generic/Materials/M_Dark.M_Dark"))))