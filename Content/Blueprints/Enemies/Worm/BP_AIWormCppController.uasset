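; AI controller Blueprint for the worm enemy, starting its behavior tree and relaying an attack command to its pawn.
; On BeginPlay it caches the controlled BP_WormPawn, sets up the BB_Worm blackboard, writes the minimum chase distance into it and runs BT_Worm.
; A HorizontalAttack event forwards to the pawn's attack, marked as temporary test code to be removed.
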(event Custom|Horizontal%20Attack
  ;[1 1 1] Esto es temporal (se va a borrar) para probar el ataque vertical
  (bind _asbp_worm_pawn (Utilities|Casting|CastToBP_WormPawn (Pawn|GetControlledPawn)))
  (Default|HorizontalAttack _asbp_worm_pawn))

(event EventBeginPlay
  (bind _asbp_worm_pawn (Utilities|Casting|CastToBP_WormPawn (Pawn|GetControlledPawn)))
  (Variables|Default|SetWormPawn _asbp_worm_pawn)
  (bind _blackboardcomponent (Class|AIController|UseBlackboard "/Game/Blueprints/Enemies/Worm/BB_Worm.BB_Worm"))
  (Variables|Default|SetBlackboard%20Component _blackboardcomponent)
  (AI|Components|Blackboard|SetValueasFloat (Variables|Default|GetBlackboard%20Component) (Variables|Default|GetMinimunDistanceToChaseName) (Variables|WormSettings|GetMinimunDistanceToChaseValue))
  (AI|RunBehaviorTree "/Game/Blueprints/Enemies/Worm/BT_Worm.BT_Worm"))

(event EventTick
  (params (DeltaSeconds :type Float%20%28single-precision%29)))

(fn ConstructionScript)