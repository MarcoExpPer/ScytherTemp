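; Mud hazard (Lodo) among the Worm enemy assets that hampers the Scyther player while inside its box.
; BeginPlay caches the player's movement and dash components plus default speed and jump values.
; Player-body overlap scales down horizontal speed, sets a reduced dash distance and, if DoesAffectJump is set, scales jump acceleration and length.
; Exit restores the cached values, but resets dash distance to a hardcoded multiplier.
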(event OnComponentBeginOverlap(Box)
  (params (OverlappedComponent :type Primitive%20Component%20Object%20Reference) (OtherActor :type Actor%20Object%20Reference) (OtherComp :type Primitive%20Component%20Object%20Reference) (OtherBodyIndex :type Integer) (bFromSweep :type Boolean) (SweepResult :type Hit%20Result%20Structure%20%28by%20ref%29))
  (if (Components|ComponentHasTag OtherComp "PlayerBody")
    (Variables|/Script/Scyther.3D_MovementComponent|SetmaxHorizontalSpeed (Variables|Default|GetMovement%20Comp) (* (Variables|/Script/Scyther.3D_MovementComponent|GetmaxHorizontalSpeed (Variables|Default|GetMovement%20Comp)) (Variables|Design|GetReductionSpeed)))
    (CallFunction|UpdateJump false)
    (Variables|/Script/Scyther.DashComponent|SetdashDistanceMultiplicator (Variables|Default|GetDash%20Component) (Variables|Design|GetReductionDash))))

(event OnComponentEndOverlap(Box)
  (params (OverlappedComponent :type Primitive%20Component%20Object%20Reference) (OtherActor :type Actor%20Object%20Reference) (OtherComp :type Primitive%20Component%20Object%20Reference) (OtherBodyIndex :type Integer))
  (if (Components|ComponentHasTag OtherComp "PlayerBody")
    (Variables|/Script/Scyther.3D_MovementComponent|SetmaxHorizontalSpeed (Variables|Default|GetMovement%20Comp) (Variables|Default|GetDefaultMaxHSpeed))
    (CallFunction|UpdateJump true)
    (Variables|/Script/Scyther.DashComponent|SetdashDistanceMultiplicator (Variables|Default|GetDash%20Component) 1e+02)))

(event EventBeginPlay
  ;[1 1 1] Save default values
  (bind _asbp_scyther_player_pawn (Utilities|Casting|CastToBP_ScytherPlayerPawn (Game|Player|GetPlayerPawn 0)))
  (bind _output_get (Variables|Default|SetMovement%20Comp (Variables|/Script/Scyther.ScytherPlayerPawn|GetmovementComp _asbp_scyther_player_pawn)))
  (Variables|Default|SetDefaultJumpAcceleration (Variables|/Script/Scyther.3D_MovementComponent|GetjumpAcceleration _output_get))
  (Variables|Default|SetDefaultJumpLength (Variables|/Script/Scyther.3D_MovementComponent|GetjumpLength (Variables|Default|GetMovement%20Comp)))
  (Variables|Default|SetDefaultMaxHSpeed (Variables|/Script/Scyther.3D_MovementComponent|GetmaxHorizontalSpeed (Variables|Default|GetMovement%20Comp)))
  (Variables|Default|SetDash%20Component (Variables|/Script/Scyther.ScytherPlayerPawn|GetdashComponent _asbp_scyther_player_pawn)))

(event EventTick
  (params (DeltaSeconds :type Float%20%28single-precision%29)))

(fn ConstructionScript)

(fn UpdateJump
  (params (toDefault :type Boolean))
  (bind _defaultjumplength (Variables|Default|GetDefaultJumpLength))
  (bind _defaultjumpacceleration (Variables|Default|GetDefaultJumpAcceleration))
  (if (Variables|Default|GetdoesAffectJump?)
    (Variables|/Script/Scyther.3D_MovementComponent|SetjumpAcceleration (Variables|Default|GetMovement%20Comp) (Math|Float|SelectFloat _defaultjumpacceleration (* _defaultjumpacceleration (Variables|Design|GetReductionJumpAceleration)) toDefault))
    (Variables|/Script/Scyther.3D_MovementComponent|SetjumpLength (Variables|Default|GetMovement%20Comp) (Math|Float|SelectFloat _defaultjumplength (* _defaultjumplength (Variables|Design|GetRedutionJumpLength)) toDefault))
    (return)
    (else
      (return))))