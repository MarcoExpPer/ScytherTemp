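; BP_newWorm is the worm enemy, handling its visual feedback and controller debugging.
; Turn-dark and turn-light events, bound on BeginPlay, swap the mesh material between Gusano_high and Gusano_high1.
; Health changes play a timeline that drives the AlphaDamage material parameter as a damage effect.
; With ActivateCtrlDebug on, Tick prints newWormCtrl's combat and current states during combat; the construction script's light-mode material logic is unconnected.
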(event HealthChangedEvent(healthComp)
  (params (oldHp :type Float%20%28single-precision%29) (newHp :type Float%20%28single-precision%29) (damageType :type DamageModes%20Enum :default "DASHEABLE"))
  ;[1 1 1] VFX_Damage
  (bind _time_damage (Timeline|Timeline_0 Play)
    (:Update
      (Rendering|Material|SetScalarParameterValueonMaterials (Variables|Default|GetwormMesh) "AlphaDamage" _time_damage))))

(event Custom|turnDarkEvent_Event_0
  (Rendering|Material|SetMaterial (Variables|Default|GetwormMesh) 0 "/Game/Arte/Escena1/Enemies/New_worm/SM_worm_without_roughness/gusano_high.gusano_high"))

(event Custom|turnLightEvent_Event_0
  (Rendering|Material|SetMaterial (Variables|Default|GetwormMesh) 0 "/Game/Arte/Escena1/Enemies/New_worm/SM_worm_without_roughness/gusano_high1.gusano_high1"))

(event EventBeginPlay
  (EventDispatchers|AssignTurnDarkEvent (delegate Custom|turnDarkEvent_Event_0))
  (EventDispatchers|AssignTurnLightEvent (delegate Custom|turnLightEvent_Event_0)))

(event Collision|EventActorBeginOverlap
  (params (OtherActor :type Actor%20Object%20Reference)))

(event EventTick
  (params (DeltaSeconds :type Float%20%28single-precision%29))
  (if (Variables|Default|GetactivateCtrlDebug)
    (bind _asnew_worm_ctrl (Utilities|Casting|CastTonewWormCtrl (Pawn|GetController)))
    (if (Utilities|Enum|Equal(Enum) (Variables|/Script/Scyther.BaseEnemyCtrl|GetcurrentCombatState _asnew_worm_ctrl) "inCombat")
      (Development|PrintString (Utilities|String|Append (Utilities|GetObjectName _asnew_worm_ctrl) " " (Utilities|String|EnumtoString (Variables|/Script/Scyther.BaseEnemyCtrl|GetcurrentCombatState _asnew_worm_ctrl)) " " (Utilities|String|EnumtoString (Variables|/Script/Scyther.newWormCtrl|GetcurrentState _asnew_worm_ctrl))) true true "(R=1.000000,G=0.069749,B=0.000000,A=1.000000)" 1e+01))))

(fn ConstructionScript)