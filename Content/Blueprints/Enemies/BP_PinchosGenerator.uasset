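; BP_PinchosGenerator is a spike trap that procedurally builds a grid of spikes and registers players standing on it for damage over time.
; The construction script places NAncho by NLargo spike meshes at InterPinchosOffset spacing, optionally hidden in game.
; It then adds a hidden plane scaled to the grid and derives the BoxColision volume from it.
; Overlaps by components tagged PlayerBody add or remove their actor in BPManualDoT.
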(event OnComponentBeginOverlap(BoxColision)
  (params (OverlappedComponent :type Primitive%20Component%20Object%20Reference) (OtherActor :type Actor%20Object%20Reference) (OtherComp :type Primitive%20Component%20Object%20Reference) (OtherBodyIndex :type Integer) (bFromSweep :type Boolean) (SweepResult :type Hit%20Result%20Structure%20%28by%20ref%29))
  (if (Components|ComponentHasTag OtherComp "PlayerBody")
    (Default|AddActor (Variables|Default|GetBP_ManualDoT) OtherActor)))

(event OnComponentEndOverlap(BoxColision)
  (params (OverlappedComponent :type Primitive%20Component%20Object%20Reference) (OtherActor :type Actor%20Object%20Reference) (OtherComp :type Primitive%20Component%20Object%20Reference) (OtherBodyIndex :type Integer))
  (if (Components|ComponentHasTag OtherComp "PlayerBody")
    (Default|RemoveActor (Variables|Default|GetBP_ManualDoT) OtherActor)))

(fn ConstructionScript
  (CallFunction|InitPinchos)
  (bind _returnvalue (AddComponent|AddStaticMeshComponent false (Math|Transform|MakeTransform (Math|Vector|MakeVector (* (Variables|Default|GetxAcumOffset) 0.5) (* (* (Variables|Default|GetnLargo) (Variables|Default|GetinterPinchosOffset)) 0.5) 5e+01) "0, 0, 0" (Math|Vector|MakeVector (Math|Conversions|ToFloat(Integer) (Variables|Default|GetnAncho)) (Math|Conversions|ToFloat(Integer) (Variables|Default|GetnLargo)) 1.0))))
  (Development|SetHiddeninGame _returnvalue true false)
  (Components|StaticMesh|SetStaticMesh _returnvalue "/Game/Arte/Escena1/Enemies/Pinchos/Mesh_Plane.Mesh_Plane")
  (bind _returnvalue_2 (AddComponent|AddBoxComponent false (Math|Transform|MakeTransform (Variables|/Script/Engine.SceneComponent|GetRelativeLocation _returnvalue) "0, 0, 0" (Math|Vector|MakeVector (* (.x (Transformation|GetWorldScale _returnvalue)) 1.5) (* (.y (Transformation|GetWorldScale _returnvalue)) 1.5) 0.1))))
  (Variables|Default|SetBoxColision _returnvalue_2))

(fn InitPinchos
  (for _index (range 0 (- (Variables|Default|GetnAncho) 1))
    (for _index_2 (range 0 (- (Variables|Default|GetnLargo) 1))
      (Utilities|CrearPinchos (+ (Variables|Default|GetxAcumOffset) (Variables|Default|GetInitialOffset)) (+ (Variables|Default|GetyAcumOffset) (Variables|Default|GetInitialOffset))
        (:exit
          (bind _output_get (Variables|Default|SetyAcumOffset (+ (stale _output_get) (Variables|Default|GetinterPinchosOffset)))))))
    (Variables|Default|SetyAcumOffset 0.0)
    (bind _output_get_2 (Variables|Default|SetxAcumOffset (+ (stale _output_get_2) (Variables|Default|GetinterPinchosOffset))))))