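; BP_Cepo is a bear trap that damages and immobilizes player or enemy bodies that overlap its box.
; When ready, it plays audio and deals damage through HealthComponent, typed dasheable or inevitable; a dasheable trap ignores targets immune to that type.
; A timeline rotates both jaws shut while the victim's 3D_MovementComponent is disabled and fixed at the trap's location.
; A timer re-arms it, resetting the jaws with a sound.
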(event OnComponentBeginOverlap(Box)
  (params (OverlappedComponent :type Primitive%20Component%20Object%20Reference) (OtherActor :type Actor%20Object%20Reference) (OtherComp :type Primitive%20Component%20Object%20Reference) (OtherBodyIndex :type Integer) (bFromSweep :type Boolean) (SweepResult :type Hit%20Result%20Structure%20%28by%20ref%29))
  (bind _returnvalue (Actor|GetComponentbyClass OtherActor "/Script/Scyther.HealthComponent"))
  (bind _returnvalue_2 (Actor|GetComponentbyClass OtherActor "/Script/Scyther.3D_MovementComponent"))
  (if (or (Components|ComponentHasTag OtherComp "PlayerBody") (Components|ComponentHasTag OtherComp "EnemyBody"))
    (if (and (Variables|Default|GetisReady?) (or (not (Variables|Default|GetisDasheable?)) (not (.Value (Utilities|Map|Find (Variables|/Script/Scyther.HealthComponent|Getinmunities _returnvalue) "DASHEABLE")))))
      ;[1 1 1] Sound Trap Activated
      (Class|FMODBlueprintStatics|PlayEvent2D "/Game/FMOD/Events/Enviroment/SFX/Trap/trapactivate.trapactivate")
      (Class|HealthComponent|ReceiveDamage _returnvalue (Variables|Default|GetonActivateDamage) (select (Variables|Default|GetisDasheable?) "DASHEABLE" "INEVITABLE") true)
      (Utilities|FlowControl|Sequence
        (:then_0
          ;[1 1 1] Animacion pocha
          (bind _newtrack_0 (Timeline|Timeline_0 PlayFromStart)
            (:Update
              (Transformation|SetRelativeRotation (Variables|Default|GetLeftSide) (Math|Rotator|Lerp(Rotator) "0, 0, 0" "0.000000, 0,75.000000" _newtrack_0) false false)
              (Transformation|SetRelativeRotation (Variables|Default|GetRightSide) (* (Math|Rotator|Lerp(Rotator) "0, 0, 0" "0.000000, 0,75.000000" _newtrack_0) -1) false false))))
        (:then_1
          ;[1 1 1] Se autoreactiva en X segundos
          (Variables|Default|SetisReady? false)
          (Utilities|Time|SetTimerbyEvent (delegate Custom|CustomEvent_0) (Variables|Default|GettimeToReactivate)))
        (:then_2
          ;[1 1 1] Disable player movement
          (Utilities|IsValid _returnvalue_2
            (:Is%20Valid
              (Class|3DMovementComponent|DisableMovementforXSeconds _returnvalue_2 (Variables|Default|GetinmovilizationTime) (Transformation|GetActorLocation)))))))))

(event Custom|CustomEvent_0
  ;[1 1 1] Se autoreactiva en X segundos
  (Variables|Default|SetisReady? true)
  (Transformation|SetRelativeRotation (Variables|Default|GetLeftSide) "0, 0, 0" false false)
  ;[1 1 1] Sound Trap Reactivated
  (Class|FMODBlueprintStatics|PlayEventatLocation "/Game/FMOD/Events/Enviroment/SFX/Trap/Trapreactive.Trapreactive" (Math|Conversions|ToTransform(Vector) (Transformation|GetActorLocation))))

(fn ConstructionScript)