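; BP_CubeEnemy is a cube enemy with a neutral, light or dark type that reacts to damage and death through its Health component.
; The construction script creates a dynamic material and colors it by EnemyType.
; Health changes play a hurt sound and shake the camera.
; At zero health it turns red, plays an explosion sound, and destroys itself after a short delay.
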(event Custom|HealthChanged
  (params (oldHp :type Float%20%28single-precision%29) (newHp :type Float%20%28single-precision%29) (damageType :type ElementTypes%20Enum :default "NEUTRAL"))
  ;[1 1 1] Cuando el enemigo recibe daño
  (Audio|PlaySoundatLocation "/Game/Audio/SFX/auch.auch" (Transformation|GetWorldLocation (Variables|Default|GetCube)) "0, 0, 0" 1.0 1.0 0.0 0 0 0)
  (Class|MatineeCameraShake|StartMatineeCameraShake (Game|GetPlayerCameraManager 0) "/Game/Blueprints/Camera/BP_ShakeEnemyHit.BP_ShakeEnemyHit_C" 1.0 "CameraLocal" "0, 0, 0"))

(event Custom|ZeroHealth
  (params (damageType :type ElementTypes%20Enum :default "NEUTRAL"))
  ;[1 1 1] Cuando el enemigo se muere
  (Rendering|Material|SetVectorParameterValue (Variables|Default|GetDinamyc%20Mat) "material" "(R=0.854902,G=0.007843,B=0.000000,A=1.000000)" :!class /Script/Engine.MaterialInstanceDynamic)
  (Audio|PlaySoundatLocation "/Game/Audio/SFX/boom.boom" (Transformation|GetWorldLocation (Variables|Default|GetCube)) "0, 0, 0" 1.0 1.0 0.0 0 0 0)
  (Utilities|FlowControl|Delay 2.8)
  (Actor|DestroyActor))

(event EventBeginPlay
  (EventDispatchers|BindEventtoHealthChangedEvent (Variables|Default|GetHealth) (delegate Custom|HealthChanged))
  (EventDispatchers|BindEventtoZerohealthEvent (Variables|Default|GetHealth) (delegate Custom|ZeroHealth)))

(fn ConstructionScript
  (bind _returnvalue (Rendering|Material|CreateDynamicMaterialInstance (Variables|Default|GetCube) 0 "/Game/Arte/Escena1/Enemies/EnemyA/Materials/mat_basic.mat_basic" "None" :!class /Script/Engine.PrimitiveComponent))
  (bind _output_get (Variables|Default|SetDinamyc%20Mat _returnvalue))
  (Rendering|Material|SetVectorParameterValue _returnvalue "material" (Utilities|Select :Index (Variables|Default|GetEnemyType) :NEUTRAL "" :LIGHT "(R=1.000000,G=0.850075,B=0.090404,A=1.000000)" :DARK "(R=0.382843,G=0.188703,B=1.000000,A=1.000000)") :!class /Script/Engine.MaterialInstanceDynamic))