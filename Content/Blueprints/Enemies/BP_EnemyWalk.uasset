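; BP_EnemyWalk is a walking enemy that chases the player until its health runs out.
; Tick re-issues AIMoveTo toward the player while alive and stops movement once dead.
; Health component events drive hit sound and camera shake, or death with a red tint, boom sound and delayed destruction.
; The construction script creates a dynamic material instance on the cylinder, colored by EnemyType.
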(event Custom|HealthChanged
  (params (oldHp :type Float%20%28single-precision%29) (newHp :type Float%20%28single-precision%29) (damageType :type ElementTypes%20Enum :default "NEUTRAL"))
  ;[1 1 1] Cuando el enemigo recibe daño
  (Audio|PlaySoundatLocation "/Game/Audio/SFX/auch.auch" (Transformation|GetWorldLocation (Variables|Default|GetCapsule)) "0, 0, 0" 1.0 1.0 0.0 0 0 0)
  (Class|MatineeCameraShake|StartMatineeCameraShake (Game|GetPlayerCameraManager 0) "/Game/Blueprints/Enemies/BP_ShakeEnemyHit.BP_ShakeEnemyHit_C" 1.0 "CameraLocal" "0, 0, 0"))

(event Custom|ZeroHealth
  (params (damageType :type ElementTypes%20Enum :default "NEUTRAL"))
  ;[1 1 1] Cuando el enemigo se muere
  (Components|DestroyComponent (Variables|Default|GetHealth))
  (Variables|Default|SetisDead? true)
  (Rendering|Material|SetVectorParameterValue (Variables|Default|Getmaterial) "material" "(R=0.854902,G=0.007843,B=0.000000,A=1.000000)" :!class /Script/Engine.MaterialInstanceDynamic)
  (Audio|PlaySoundatLocation "/Game/Audio/SFX/boom.boom" (Transformation|GetWorldLocation (Variables|Default|GetCapsule)) "0, 0, 0" 1.0 1.0 0.0 0 0 0)
  (Utilities|FlowControl|Delay 2.8)
  (Actor|DestroyActor))

(event EventBeginPlay
  (EventDispatchers|BindEventtoHealthChangedEvent (Variables|Default|GetHealth) (delegate Custom|HealthChanged))
  (EventDispatchers|BindEventtoZerohealthEvent (Variables|Default|GetHealth) (delegate Custom|ZeroHealth)))

(event Collision|EventActorBeginOverlap
  (params (OtherActor :type Actor%20Object%20Reference)))

(event EventTick
  (params (DeltaSeconds :type Float%20%28single-precision%29))
  (if (Variables|Default|GetisDead?)
    (Components|Movement|StopMovementImmediately (Variables|Character|GetCharacterMovement))
    (else
      ;[1 1 1] Movemos el enemigo hacia el jugador
      (Utilities|IsValid (Variables|Default|GetHealth)
        (:Is%20Valid
          (AI|AIMoveTo self "0, 0, 0" (Game|GetPlayerCharacter 0) 1e+01 false))))))

(fn ConstructionScript
  ;[1 1 1] Darle un color básico al cubo
  (bind _returnvalue (Rendering|Material|CreateDynamicMaterialInstance (Variables|Default|GetCylinder) 0 "/Game/Arte/Escena1/Enemies/EnemyA/Materials/mat_basic.mat_basic" "None" :!class /Script/Engine.PrimitiveComponent))
  (Variables|Default|Setmaterial _returnvalue)
  (if (Utilities|Enum|Equal(Enum) (Variables|Default|GetEnemyType) "LIGHT")
    (Rendering|Material|SetVectorParameterValue (Variables|Default|Getmaterial) "material" "(R=0.859375,G=0.775044,B=0.182579,A=1.000000)" :!class /Script/Engine.MaterialInstanceDynamic)
    (else
      (Rendering|Material|SetVectorParameterValue (Variables|Default|Getmaterial) "material" "(R=0.037461,G=0.006405,B=0.208333,A=1.000000)" :!class /Script/Engine.MaterialInstanceDynamic))))