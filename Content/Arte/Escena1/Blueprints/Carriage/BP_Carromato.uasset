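; BP_Carromato is a carriage actor for Escena1 that fades out while the player is inside a trigger box around or near it.
; The HideMeshWhenInsideThisBox overlap events set a Disappear flag for components tagged PlayerBody.
; Tick steps Opacity down toward a minimum or back up to one, independent of delta time, and writes it to the Destructible component's material parameter.
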(event OnComponentBeginOverlap(HideMeshWhenInsideThisBox)
  (params (OverlappedComponent :type Primitive%20Component%20Object%20Reference) (OtherActor :type Actor%20Object%20Reference) (OtherComp :type Primitive%20Component%20Object%20Reference) (OtherBodyIndex :type Integer) (bFromSweep :type Boolean) (SweepResult :type Hit%20Result%20Structure%20%28by%20ref%29))
  (if (Components|ComponentHasTag OtherComp "PlayerBody")
    (Variables|Default|SetDisappear true)))

(event OnComponentEndOverlap(HideMeshWhenInsideThisBox)
  (params (OverlappedComponent :type Primitive%20Component%20Object%20Reference) (OtherActor :type Actor%20Object%20Reference) (OtherComp :type Primitive%20Component%20Object%20Reference) (OtherBodyIndex :type Integer))
  (if (Components|ComponentHasTag OtherComp "PlayerBody")
    (Variables|Default|SetDisappear false)))

(event EventBeginPlay
  (|CallParentFunction) ; This node is disabled and will not be called.\nDrag off pins to build functionality.
)

(event Collision|EventActorBeginOverlap
  (params (OtherActor :type Actor%20Object%20Reference)))

(event EventTick
  (params (DeltaSeconds :type Float%20%28single-precision%29))
  (bind _decreasestep (Variables|Default|GetdecreaseStep))
  (|CallParentFunction 0.0)
  (if (Variables|Default|GetDisappear)
    (if (> (Variables|Default|GetOpacity) (Variables|Default|GetminimumOpactiy))
      (Variables|Default|SetOpacity (- (Variables|Default|GetOpacity) _decreasestep))
      (Rendering|Material|SetScalarParameterValueonMaterials (Variables|Default|GetDestructible) "Opacity" (Variables|Default|GetOpacity) :!label _label))
    (elif (< (Variables|Default|GetOpacity) 1.0)
      (Variables|Default|SetOpacity (+ (Variables|Default|GetOpacity) _decreasestep))
      (goto _label))))

(fn ConstructionScript
  (|CallParentFunction))