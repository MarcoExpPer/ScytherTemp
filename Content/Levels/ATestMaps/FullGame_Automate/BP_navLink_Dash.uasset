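; BP_navLink_Dash is a nav-link helper actor that makes an AI-controlled Scyther player dash when it enters either of two box triggers.
; Both box overlaps call MakeAIPawnJump, which checks for the PlayerBody component tag and calls DoDash on BP_ScytherPlayer_AI_Controller, despite the function's jump name.
; An IsInUse flag is set after the dash and never reset here, so each instance triggers once.
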(event OnComponentBeginOverlap(Box)
  (params (OverlappedComponent :type Primitive%20Component%20Object%20Reference) (OtherActor :type Actor%20Object%20Reference) (OtherComp :type Primitive%20Component%20Object%20Reference) (OtherBodyIndex :type Integer) (bFromSweep :type Boolean) (SweepResult :type Hit%20Result%20Structure%20%28by%20ref%29))
  (CallFunction|MakeAIPawnJump OtherComp OtherActor))

(event OnComponentBeginOverlap(Box1)
  (params (OverlappedComponent :type Primitive%20Component%20Object%20Reference) (OtherActor :type Actor%20Object%20Reference) (OtherComp :type Primitive%20Component%20Object%20Reference) (OtherBodyIndex :type Integer) (bFromSweep :type Boolean) (SweepResult :type Hit%20Result%20Structure%20%28by%20ref%29))
  (CallFunction|MakeAIPawnJump OtherComp OtherActor))

(event EventBeginPlay)

(event Collision|EventActorBeginOverlap
  (params (OtherActor :type Actor%20Object%20Reference)))

(event EventTick
  (params (DeltaSeconds :type Float%20%28single-precision%29)))

(fn ConstructionScript)

(fn MakeAIPawnJump
  (params (Component :type Actor%20Component%20Object%20Reference) (OwnerActor :type Actor%20Object%20Reference))
  (if (and (Components|ComponentHasTag Component "PlayerBody") (not (Variables|Default|GetisInUse)))
    (bind _asbp_scyther_player_ai_controller (Utilities|Casting|CastToBP_ScytherPlayer_AI_Controller (AI|GetAIController OwnerActor))
      (:then
        (Default|DoDash _asbp_scyther_player_ai_controller)
        (Variables|Default|SetisInUse true)
        (return))
      (:CastFailed
        _)))
  (return))