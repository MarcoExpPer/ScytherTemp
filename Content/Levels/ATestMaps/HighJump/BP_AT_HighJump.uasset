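; Automated functional test that checks whether the Scyther player can jump and travel right in the high jump test map.
; PrepareTest casts the player controller, moves the pawn to the PlayerStart, records its X position and becomes ready after a short delay.
; StartTest triggers a jump, while Tick simulates right movement and passes once the pawn covers a set X distance.
; A failed controller cast ends the test with an error.
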(event EventPrepareTest
  (bind _asscyther_player_controller (Utilities|Casting|CastToScytherPlayerController (Game|GetPlayerController 0))
    (:then
      (Variables|Default|SetAs%20Scyther%20Player%20Controller _asscyther_player_controller)
      (bind _returnvalue (Actor|GetActorOfClass "/Script/Engine.PlayerStart"))
      (Transformation|SetActorLocation (Game|Player|GetPlayerPawn 0) (Transformation|GetActorLocation _returnvalue) false false)
      (Variables|Default|SetstartingX (.x (Transformation|GetActorLocation (Game|Player|GetPlayerPawn 0))))
      (Utilities|FlowControl|Delay 0.5)
      (Variables|Default|SetisReady? true))
    (:CastFailed
      (Class|FunctionalTest|FinishTest "Error" "ScytherPlayerController cast failed"))))

(event EventTick
  (params (DeltaSeconds :type Float%20%28single-precision%29))
  (if (Variables|Default|GetisReady?)
    (Class|ScytherPlayerController|CallMoveRight (Variables|Default|GetAs%20Scyther%20Player%20Controller) 1.0)
    (if (>= (.x (Transformation|GetActorLocation (Game|Player|GetPlayerPawn 0))) (+ (Variables|Default|GetstartingX) 4e+02))
      (Class|FunctionalTest|FinishTest "Succeeded"))))

(event EventStartTest
  (Class|ScytherPlayerController|CallJumpPressed (Variables|Default|GetAs%20Scyther%20Player%20Controller))
  (Development|PrintString "Hello"))

(fn ConstructionScript)

(fn IsReady
  (return (Variables|Default|GetisReady?)))