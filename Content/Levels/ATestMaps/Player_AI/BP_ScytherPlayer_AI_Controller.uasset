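; AI controller that plays the Scyther player pawn automatically, topping it up to very high health on start.
; CombatZone events switch it between combat, which runs a behavior tree, and navmesh path following toward TargetLocation, which idles at path end.
; Tick steers toward the combat location or next path point through the pawn's player movement functions.
; Helper events trigger jumps, queued attacks, light skill and dashes that retry until available.
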(event Custom|CombatStartsEvent_Event_0
  (CallFunction|StartCombatMode))

(event Custom|MovementTick
  (params (deltaTime :type Float%20%28single-precision%29))
  (bind _movementpath (Variables|Movement|GetmovementPath))
  (bind _currentpathindex (Variables|Movement|GetcurrentPathIndex))
  (bind _movementpath_2 (Variables|Movement|GetmovementPath))
  (bind _currentpathindex_2 (Variables|Movement|GetcurrentPathIndex))
  (bind _as_bp_scyther_player_pawn_ai (Variables|Default|GetAs%20BP%20Scyther%20Player%20Pawn%20AI))
  (bind _as_bp_scyther_player_pawn_ai_2 (Variables|Default|GetAs%20BP%20Scyther%20Player%20Pawn%20AI))
  (bind _as_bp_scyther_player_pawn_ai_3 (Variables|Default|GetAs%20BP%20Scyther%20Player%20Pawn%20AI))
  (bind _returnvalue (Transformation|GetActorLocation _as_bp_scyther_player_pawn_ai_3))
  (bind _returnvalue_2 (Transformation|GetActorLocation _as_bp_scyther_player_pawn_ai_2))
  (bind _output (Utilities|Array|Get(acopy) _movementpath _currentpathindex))
  (bind _output_2 (Utilities|Array|Get(acopy) _movementpath_2 _currentpathindex_2))
  (bind _returnvalue_3 (- _output _returnvalue))
  (bind _returnvalue_4 (Class|KismetMathLibrary|VectorNormal2D _returnvalue_3 0.0001))
  (if (Math|Vector|Equal(Vector) (Math|Vector|MakeVector (.x _output_2) (.y _output_2) (.z _output_2)) (Math|Vector|MakeVector (.x _returnvalue_2) (.y _returnvalue_2) (.z _output_2)) 5e+01)
    (CallFunction|CalculateNextPathLocation)
    (else
      (Class|ScytherPlayerPawn|MoveRight _as_bp_scyther_player_pawn_ai (.x _returnvalue_4))
      (Class|ScytherPlayerPawn|MoveForward _as_bp_scyther_player_pawn_ai (* (.y _returnvalue_4) -1.0)))))

(event Custom|UseSkill
  (bind _as_bp_scyther_player_pawn_ai (Variables|Default|GetAs%20BP%20Scyther%20Player%20Pawn%20AI))
  (bind _skillcomponent (Variables|/Script/Scyther.ScytherPlayerPawn|GetskillComponent _as_bp_scyther_player_pawn_ai))
  (Class|SkillComponent|UpdateMana _skillcomponent true 1e+02)
  (Class|SkillComponent|EnableLightSkill _skillcomponent))

(event Custom|DoJump
  (params (jumpPressDuration :type Float%20%28single-precision%29))
  (bind _as_bp_scyther_player_pawn_ai (Variables|Default|GetAs%20BP%20Scyther%20Player%20Pawn%20AI))
  (Class|ScytherPlayerPawn|OnJumpPressed _as_bp_scyther_player_pawn_ai)
  (Utilities|FlowControl|Delay jumpPressDuration)
  (Class|ScytherPlayerPawn|OnJumpReleased _as_bp_scyther_player_pawn_ai))

(event Custom|DoDash
  (Variables|Default|SetAIstate "NewEnumerator2")
  (bind _returnvalue (Class|DashComponent|CheckDashAvailable (Variables|/Script/Scyther.ScytherPlayerPawn|GetdashComponent (Variables|Default|GetAs%20BP%20Scyther%20Player%20Pawn%20AI)) :!label _label))
  (if _returnvalue
    (Class|ScytherPlayerPawn|OnDash (Variables|Default|GetAs%20BP%20Scyther%20Player%20Pawn%20AI))
    (Variables|Default|SetAIstate "NewEnumerator0")
    (else
      (Utilities|FlowControl|Delay 0.5)
      (goto _label))))

(event Custom|DoOneAttack
  (if (> (Variables|Movement|GetattacksLeftToDo) 0)
    (Class|ScytherPlayerPawn|OnAttack (Variables|Default|GetAs%20BP%20Scyther%20Player%20Pawn%20AI))
    (Math|Integer|DecrementInt (Variables|Movement|GetattacksLeftToDo)
      (:%20%20
        (if (> (Variables|Movement|GetattacksLeftToDo) 0)
          (Class|ScytherPlayerPawn|OnAttack (Variables|Default|GetAs%20BP%20Scyther%20Player%20Pawn%20AI))
          (Math|Integer|DecrementInt (Variables|Movement|GetattacksLeftToDo)))))))

(event Custom|StartCombatMode
  (Development|PrintString "Combat Mode On")
  (AI|RunBehaviorTree "/Game/Levels/ATestMaps/Player_AI/BTT_PlayerCombat.BTT_PlayerCombat")
  (Variables|Default|SetAIstate "NewEnumerator1"))

(event Custom|StartMovementMode
  (Development|PrintString "Movement Mode On")
  (CallFunction|GetPathtoTargetLocation)
  (Variables|Default|SetAIstate "NewEnumerator0"))

(event Custom|CustomEvent_0
  (CallFunction|StartMovementMode))

(event Custom|StartIdleMode
  (Development|PrintString "Idle Mode On")
  (Variables|Default|SetAIstate "NewEnumerator2"))

(event Custom|GetPathToTargetLocation
  (bind _returnvalue (Class|NavigationSystemV1|FindPathtoLocationSynchronously (Transformation|GetActorLocation (Pawn|GetControlledPawn)) (Variables|Movement|GettargetLocation) self 0))
  (Class|NavigationPath|EnableDebugDrawing _returnvalue true "(R=1.000000,G=0.000000,B=0.972670,A=1.000000)")
  (Variables|Movement|SetmovementPath (Variables|/Script/NavigationSystem.NavigationPath|GetPathPoints _returnvalue))
  (Variables|Movement|SetcurrentPathIndex 1))

(event Custom|CombatTick
  (params (deltaTime :type Float%20%28single-precision%29))
  (bind _as_bp_scyther_player_pawn_ai (Variables|Default|GetAs%20BP%20Scyther%20Player%20Pawn%20AI))
  (bind _locationtomovetoincombat (Variables|Combat|GetlocationToMoveToInCombat))
  (bind _as_bp_scyther_player_pawn_ai_2 (Variables|Default|GetAs%20BP%20Scyther%20Player%20Pawn%20AI))
  (bind _returnvalue (Transformation|GetActorLocation _as_bp_scyther_player_pawn_ai_2))
  (bind _returnvalue_2 (- _locationtomovetoincombat _returnvalue))
  (bind _returnvalue_3 (Class|KismetMathLibrary|VectorNormal2D _returnvalue_2 0.0001))
  (if (not (Math|Vector|Equal(Vector) (Variables|Combat|GetlocationToMoveToInCombat) (Transformation|GetActorLocation (Variables|Default|GetAs%20BP%20Scyther%20Player%20Pawn%20AI)) 5e+01))
    (Class|ScytherPlayerPawn|MoveRight _as_bp_scyther_player_pawn_ai (.x _returnvalue_3))
    (Class|ScytherPlayerPawn|MoveForward _as_bp_scyther_player_pawn_ai (* (.y _returnvalue_3) -1.0))))

(event Custom|CustomEvent_1
  (if (Utilities|Enum|Equal(Enum) (Variables|Default|GetAIstate) "NewEnumerator0")
    (CallFunction|DoOneAttack)))

(event Custom|CalculateNextPathLocation
  (if (>= (Variables|Movement|GetcurrentPathIndex) (- (Utilities|Array|Length (Variables|Movement|GetmovementPath)) 1))
    (Development|PrintString "End of path")
    (CallFunction|StartIdleMode)
    (else
      (Math|Integer|IncrementInt (Variables|Movement|GetcurrentPathIndex)))))

(event EventBeginPlay
  (bind _asbp_scyther_player_pawn_ai (Utilities|Casting|CastToBP_ScytherPlayerPawn_AI (Pawn|GetControlledPawn)))
  (bind _output_get (Variables|Default|SetAs%20BP%20Scyther%20Player%20Pawn%20AI _asbp_scyther_player_pawn_ai))
  (bind _output_get_2 (Variables|/Script/Scyther.HealthComponent|SetmaxHp (Variables|/Script/Scyther.ScytherPlayerPawn|GethealthComponent _output_get) 99999.0))
  (Class|HealthComponent|ChangeHealth (Variables|/Script/Scyther.ScytherPlayerPawn|GethealthComponent _output_get) _output_get_2 "HEALING" true)
  (EventDispatchers|BindEventtoAttackFinishedEvent (Variables|/Script/Scyther.ScytherPlayerPawn|GetattackComponent _output_get) (delegate Custom|CustomEvent_1))
  (Variables|Combat|SetlocationToMoveToInCombat (Transformation|GetActorLocation (Variables|Default|GetAs%20BP%20Scyther%20Player%20Pawn%20AI)))
  (bind _outactors (Actor|GetAllActorsOfClass "/Script/Scyther.CombatZone"))
  (for _array_element _outactors
    (EventDispatchers|AssignCombatStartsEvent _array_element (delegate Custom|CombatStartsEvent_Event_0))
    (EventDispatchers|BindEventtoCombatEndsEvent _array_element (delegate Custom|CustomEvent_0))))

(event EventTick
  (params (DeltaSeconds :type Float%20%28single-precision%29))
  (switch Utilities|FlowControl|Switch|SwitchonPlayerAIStates (Variables|Default|GetAIstate)
    (:NewEnumerator0
      (CallFunction|MovementTick 0.0))
    (:NewEnumerator1
      (CallFunction|CombatTick DeltaSeconds))))

(fn ConstructionScript)