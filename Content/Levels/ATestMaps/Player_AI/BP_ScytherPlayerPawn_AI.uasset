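; AI-driven variant of the Scyther player pawn, apparently for AI test maps, that starts in either movement or combat mode.
; On BeginPlay it hides its circle ring and entity shadows, then passes the location of InitialMovementTarget to its BP_ScytherPlayer_AI_Controller.
; After a short delay, InitialMode selects whether the controller starts movement mode (out of combat) or combat mode.
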(event EventBeginPlay
  (|CallParentFunction)
  (Development|SetHiddeninGame (Variables|Default|GetcircleRingShadow) true false)
  (Development|SetHiddeninGame (Variables|Default|GetentityShadow) true false)
  (bind _asbp_scyther_player_ai_controller (Utilities|Casting|CastToBP_ScytherPlayer_AI_Controller (Pawn|GetController)))
  (Variables|/Game/Levels/ATestMaps/Player_AI/BP_ScytherPlayer_AI_Controller.BP_ScytherPlayer_AI_Controller_C|SettargetLocation _asbp_scyther_player_ai_controller (Transformation|GetActorLocation (Variables|Default|GetinitialMovementTarget)))
  (Utilities|FlowControl|Delay 2.0)
  (switch Utilities|FlowControl|Switch|SwitchonPlayerAIStates (Variables|Default|GetinitialMode)
    (:NewEnumerator0
      (Default|StartMovementMode _asbp_scyther_player_ai_controller))
    (:NewEnumerator1
      (Default|StartCombatMode _asbp_scyther_player_ai_controller))))

(event Collision|EventActorBeginOverlap
  (params (OtherActor :type Actor%20Object%20Reference))
  (|CallParentFunction OtherActor) ; This node is disabled and will not be called.\nDrag off pins to build functionality.
)

(event EventTick
  (params (DeltaSeconds :type Float%20%28single-precision%29))
  (|CallParentFunction DeltaSeconds) ; This node is disabled and will not be called.\nDrag off pins to build functionality.
)

(fn ConstructionScript
  (|CallParentFunction))