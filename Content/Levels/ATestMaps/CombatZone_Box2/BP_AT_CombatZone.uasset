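; Functional test that checks an AI-driven Scyther player can clear a tagged combat zone before a timeout.
; Setup finds the AI controller, pawn and zone, binds the combat-end event and waits briefly before reporting ready.
; Tick walks the pawn right whenever it is out of combat; combat ending passes the test.
; A timeout fails it, reporting the current round and each surviving rabbit or worm's health, plus location for worms.
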(event Custom|CustomEvent_0
  (Class|FunctionalTest|FinishTest "Succeeded" "Combat finished"))

(event Custom|CustomEvent_1
  (bind _errormsg (CallFunction|GetFinishErrorMsg (Variables|Default|GetCombatZone)))
  (Class|FunctionalTest|FinishTest "Failed" (Utilities|String|Append " 
TIMEOUT: 
" _errormsg)))

(event EventPrepareTest
  (bind _returnvalue (Actor|GetActorOfClass "/Game/Levels/ATestMaps/CombatZone_Box2/BP_ScytherPlayer_AI_Controller.BP_ScytherPlayer_AI_Controller_C"))
  (Variables|Default|SetScytherController_AI _returnvalue)
  (bind _returnvalue_2 (Actor|GetActorOfClass "/Game/Levels/ATestMaps/CombatZone_Box2/BP_ScytherPlayerPawn_AI.BP_ScytherPlayerPawn_AI_C"))
  (Variables|Default|SetScytherPawn_AI _returnvalue_2)
  (bind _outactors (Actor|GetAllActorswithTag (Variables|Default|GetTagOfTheCombatZone)))
  (bind _asbp_combat_zone (Utilities|Casting|CastToBP_CombatZone (Utilities|Array|Get(acopy) _outactors)))
  (bind _output_get (Variables|Default|SetCombatZone _asbp_combat_zone))
  (EventDispatchers|BindEventtoCombatEndsEvent _output_get (delegate Custom|CustomEvent_0))
  (Utilities|FlowControl|Delay 2.0)
  (Variables|Default|SetisReady? true))

(event EventTick
  (params (DeltaSeconds :type Float%20%28single-precision%29))
  (if (and (not (Variables|/Game/Levels/ATestMaps/CombatZone_Box2/BP_ScytherPlayer_AI_Controller.BP_ScytherPlayer_AI_Controller_C|GetisInCombat? (Variables|Default|GetScytherController_AI))) (Variables|Default|GetisReady?))
    (Class|ScytherPlayerPawn|MoveRight (Variables|Default|GetScytherPawn_AI) 1.0)))

(event EventStartTest
  (bind _returnvalue (Utilities|Time|SetTimerbyEvent (delegate Custom|CustomEvent_1) (Variables|Default|Gettimeout)))
  (Variables|Default|SettimeoutHandle _returnvalue))

(fn ConstructionScript)

(fn IsReady
  (return (Variables|Default|GetisReady?)))

(fn GetFinishErrorMsg
  (params (CombatZone :type Combat%20Zone%20Object%20Reference))
  (bind _currentround (Variables|/Script/Scyther.CombatZone|GetcurrentRound CombatZone))
  (LocalVariables|Setmsg (Utilities|String|Append "Current Combat Round: " (Utilities|String|ToString(Integer) _currentround) " 
 
"))
  (for _array_element (Variables|/Script/Scyther.CombatRoundPoint|GetenemiesPawns (Utilities|Array|Get(acopy) (Variables|/Script/Scyther.CombatZone|Getrounds CombatZone) _currentround))
    (if (not (Variables|/Script/Scyther.BaseEnemy|GetisDead _array_element))
      (bind _asbp_new_rabbit (Utilities|Casting|CastToBP_NewRabbit _array_element)
        (:then
          (bind _newparam (CallFunction|GetRabbitErrorMsg _asbp_new_rabbit))
          (LocalVariables|Setmsg (Utilities|String|Append (LocalVariables|Getmsg) _newparam)))
        (:CastFailed
          (bind _asbp_worm_pawn (Utilities|Casting|CastToBP_WormPawn _array_element))
          (bind _msg (CallFunction|GetWormErrorMsg _asbp_worm_pawn))
          (LocalVariables|Setmsg (Utilities|String|Append (LocalVariables|Getmsg) _msg))))))
  (return (LocalVariables|Getmsg)))

(fn GetRabbitErrorMsg
  (params (rabbit :type BP%20New%20Rabbit%20Object%20Reference))
  (bind _healthcomp (Variables|/Script/Scyther.BaseEnemy|GethealthComp rabbit))
  (return (Utilities|String|Append (Utilities|GetDisplayName rabbit) " has " (Utilities|String|ToString(Float) (Variables|/Script/Scyther.HealthComponent|GetcurrentHp _healthcomp)) " hp out of " (Utilities|String|ToString(Float) (Variables|/Script/Scyther.HealthComponent|GetmaxHp _healthcomp)) "hp 
")))

(fn GetWormErrorMsg
  (params (Worm :type BP%20Worm%20Pawn%20Object%20Reference))
  (bind _healthcomp (Variables|/Script/Scyther.BaseEnemy|GethealthComp Worm))
  (return (Utilities|String|Append (Utilities|GetDisplayName Worm) " has " (Utilities|String|ToString(Float) (Variables|/Script/Scyther.HealthComponent|GetcurrentHp _healthcomp)) " hp out of " (Utilities|String|ToString(Float) (Variables|/Script/Scyther.HealthComponent|GetmaxHp _healthcomp)) "hp, location = " (Utilities|String|ToString(Vector) (Transformation|GetActorLocation Worm)) " 
")))