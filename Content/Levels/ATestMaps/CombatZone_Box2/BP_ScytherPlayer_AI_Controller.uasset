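; AI controller for the Scyther player's AI-driven pawn in the CombatZone_Box2 test map.
; On BeginPlay it caches the pawn and sets the move target to its current location.
; StartBTT runs the BTT_PlayerCombat behavior tree and activates steering.
; While active, Tick feeds the normalized 2D direction toward LocationToMoveTo into the pawn's MoveRight and MoveForward (Y negated), bypassing navigation pathing until within tolerance.
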(event Custom|StartBTT
  (AI|RunBehaviorTree "/Game/Levels/ATestMaps/CombatZone_Box2/BTT_PlayerCombat.BTT_PlayerCombat")
  (Variables|Default|SetisActive? true))

(event EventBeginPlay
  (bind _asbp_scyther_player_pawn_ai (Utilities|Casting|CastToBP_ScytherPlayerPawn_AI (Pawn|GetControlledPawn)))
  (Variables|Default|SetAs%20BP%20Scyther%20Player%20Pawn%20AI _asbp_scyther_player_pawn_ai)
  (Variables|Default|SetlocationToMoveTo (Transformation|GetActorLocation (Variables|Default|GetAs%20BP%20Scyther%20Player%20Pawn%20AI))))

(event EventTick
  (params (DeltaSeconds :type Float%20%28single-precision%29))
  (bind _as_bp_scyther_player_pawn_ai (Variables|Default|GetAs%20BP%20Scyther%20Player%20Pawn%20AI))
  (bind _as_bp_scyther_player_pawn_ai_2 (Variables|Default|GetAs%20BP%20Scyther%20Player%20Pawn%20AI))
  (bind _locationtomoveto (Variables|Default|GetlocationToMoveTo))
  (bind _returnvalue (Transformation|GetActorLocation _as_bp_scyther_player_pawn_ai_2))
  (bind _returnvalue_2 (- _locationtomoveto _returnvalue))
  (bind _returnvalue_3 (Class|KismetMathLibrary|VectorNormal2D _returnvalue_2 0.0001))
  (if (Variables|Default|GetisActive?)
    (if (not (Math|Vector|Equal(Vector) (Variables|Default|GetlocationToMoveTo) (Transformation|GetActorLocation (Variables|Default|GetAs%20BP%20Scyther%20Player%20Pawn%20AI)) 5e+01))
      (Class|ScytherPlayerPawn|MoveRight _as_bp_scyther_player_pawn_ai (.x _returnvalue_3))
      (Class|ScytherPlayerPawn|MoveForward _as_bp_scyther_player_pawn_ai (* (.y _returnvalue_3) -1.0)))))

(fn ConstructionScript)