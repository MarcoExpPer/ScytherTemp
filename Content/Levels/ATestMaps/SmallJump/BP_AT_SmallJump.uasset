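; BP_AT_SmallJump is an automated functional test for a short jump while moving right, driven through the Scyther player controller.
; Preparation moves the pawn to the PlayerStart, records its X position and marks the test ready after a delay.
; Tick then holds right input while the test start simulates a brief jump tap.
; The test succeeds once the pawn travels a set X distance, with no explicit failure branch.
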(event EventPrepareTest
  (bind _asbp_scyther_player_controller (Utilities|Casting|CastToBP_ScytherPlayerController (Game|GetPlayerController 0)))
  (Variables|Default|SetAs%20BP%20Scyther%20Player%20Controller _asbp_scyther_player_controller)
  (bind _returnvalue (Actor|GetActorOfClass "/Script/Engine.PlayerStart"))
  (Transformation|SetActorLocation (Game|Player|GetPlayerPawn 0) (Transformation|GetActorLocation _returnvalue) false false)
  (Variables|Default|SetstartingX (.x (Transformation|GetActorLocation (Game|Player|GetPlayerPawn 0))))
  (Utilities|FlowControl|Delay 0.5)
  (Variables|Default|SetisReady? true))

(event EventTick
  (params (DeltaSeconds :type Float%20%28single-precision%29))
  (if (Variables|Default|GetisReady?)
    (Class|ScytherPlayerController|CallMoveRight (Variables|Default|GetAs%20BP%20Scyther%20Player%20Controller) 1.0)
    (if (>= (.x (Transformation|GetActorLocation (Game|Player|GetPlayerPawn 0))) (+ (Variables|Default|GetstartingX) 4e+02))
      (Class|FunctionalTest|FinishTest "Succeeded"))))

(event EventStartTest
  (bind _as_bp_scyther_player_controller (Variables|Default|GetAs%20BP%20Scyther%20Player%20Controller))
  (Utilities|FlowControl|Delay 0.5)
  (Class|ScytherPlayerController|CallJumpPressed _as_bp_scyther_player_controller)
  (Utilities|FlowControl|Delay 0.01)
  (Class|ScytherPlayerController|CallJumpReleased _as_bp_scyther_player_controller))

(fn ConstructionScript)

(fn IsReady
  (return (Variables|Default|GetisReady?)))