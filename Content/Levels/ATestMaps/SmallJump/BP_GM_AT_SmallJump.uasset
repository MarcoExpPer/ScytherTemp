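; Game mode for the SmallJump test map that starts the game through BP_GameInstance and handles death and respawn audio.
; After a short BeginPlay delay it binds to the RespawnMan death and respawn events, each playing a 2D sound.
; Death also mutes gameplay audio buses, fades out final combat audio and changes the music via the game instance.
; Helpers unmute most buses, though nothing here calls that, and broadcast gamepad-use changes.
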(event Custom|PlayerDeath
  ;[1 1 1] Estaría bien, si tenemos sonidos de muerte poner un sonido de muerte cuando el personaje muere (rollo SFX de muerte como Dark Souls) y que se deje de escuchar la música
  (Class|FMODBlueprintStatics|PlayEvent2D "/Game/FMOD/Events/Music/UI/Death/Death.Death")
  (CallFunction|DisableVolume)
  (Utilities|IsValid (Variables|Audio|GetBP%20Game%20Instance)
    (:Is%20Valid
      _)
    (:Is%20Not%20Valid
      (bind _asbp_game_instance (Utilities|Casting|CastToBP_GameInstance (Game|GetGameInstance)))
      (bind _output_get (Variables|Audio|SetBP%20Game%20Instance _asbp_game_instance))))
  (Default|ChangeGameMusic _output_get 3.0))

(event Custom|PlayerRespawn
  (params (location :type Vector))
  ;[1 1 1] When you die, the combat music return to de prado music (Respawn)
  (Class|FMODBlueprintStatics|PlayEvent2D "/Game/FMOD/Events/Player/Respawn/Respawn.Respawn"))

(event EventBeginPlay
  (bind _respawnman (Variables|Default|GetrespawnMan))
  (|CallParentFunction)
  (bind _asbp_game_instance (Utilities|Casting|CastToBP_GameInstance (Game|GetGameInstance)))
  (Default|StartGame _asbp_game_instance)
  (Utilities|FlowControl|Delay 0.2)
  (EventDispatchers|BindEventtoPlayerDeadEvent _respawnman (delegate Custom|PlayerDeath))
  (EventDispatchers|BindEventtoPlayerRespawnEvent _respawnman (delegate Custom|PlayerRespawn)))

(fn ConstructionScript)

(fn ChangeIsUsingGamepad
  (params (newValue :type Boolean))
  (if (Math|Boolean|NotEqual(Boolean) newValue (Variables|Default|GetisUsingGamepad?))
    (bind _output_get (Variables|Default|SetisUsingGamepad? (not (Variables|Default|GetisUsingGamepad?))))
    (Default|CallIsUsingGamepadUpdated _output_get)))

(fn DisableVolume
  (Class|FMODBlueprintStatics|BusSetMute "/Game/FMOD/Buses/GameSFX/Enviroment_Sounds/Ambient.Ambient" true)
  (Class|FMODBlueprintStatics|BusSetMute "/Game/FMOD/Buses/GameMusic/PradoLevel.PradoLevel" true)
  (Class|FMODBlueprintStatics|BusSetMute "/Game/FMOD/Buses/GameSFX.GameSFX" true)
  (Class|FMODBlueprintStatics|BusSetMute "/Game/FMOD/Buses/UI/ZTarget.ZTarget" true)
  (Class|FMODBlueprintStatics|BusSetMute "/Game/FMOD/Buses/UI/Lootables.Lootables" true)
  (Class|FMODBlueprintStatics|BusStopAllEvents "/Game/FMOD/Buses/GameMusic/FinalCombat.FinalCombat" "ALLOWFADEOUT"))

(fn ActivateVolume
  (Class|FMODBlueprintStatics|BusSetMute "/Game/FMOD/Buses/GameSFX/Enviroment_Sounds/Ambient.Ambient" false)
  (Class|FMODBlueprintStatics|BusSetMute "/Game/FMOD/Buses/GameMusic/PradoLevel.PradoLevel" false)
  (Class|FMODBlueprintStatics|BusSetMute "/Game/FMOD/Buses/UI/ZTarget.ZTarget" false)
  (Class|FMODBlueprintStatics|BusSetMute "/Game/FMOD/Buses/UI/Lootables.Lootables" false))