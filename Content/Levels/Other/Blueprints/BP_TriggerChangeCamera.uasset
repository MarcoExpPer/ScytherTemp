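; Trigger volume that switches the game camera between normal, side-scroll and combat-enemy modes.
; When a component tagged PlayerBody overlaps the box, it sets the referenced camera's mode to the trigger's type if different.
; Each mode rotates the camera root from its own direction vector.
; Normal and side-scroll also shift the referenced spline by opposite Y/Z offsets to reposition the camera, while combat leaves the spline untouched.
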(event OnComponentBeginOverlap(TriggerBox(CollisionBox))
  (params (OverlappedComponent :type Primitive%20Component%20Object%20Reference) (OtherActor :type Actor%20Object%20Reference) (OtherComp :type Primitive%20Component%20Object%20Reference) (OtherBodyIndex :type Integer) (bFromSweep :type Boolean) (SweepResult :type Hit%20Result%20Structure%20%28by%20ref%29))
  (bind _refspline (Variables|Default|GetRefSpline))
  (bind _refcamera (Variables|Default|GetRefCamera))
  (bind _typecamera (Variables|Default|GetTypeCamera))
  (bind _rootcomponent (Variables|/Script/Engine.Actor|GetRootComponent _refspline))
  (bind _returnvalue (Transformation|GetWorldLocation _rootcomponent))
  (if (Components|ComponentHasTag OtherComp "PlayerBody")
    (if (Utilities|Enum|NotEqual(Enum) (Variables|/Game/Blueprints/Player/Camera/BP_CameraRail.BP_CameraRail_C|GetmodeTypeCamera (Variables|Default|GetRefCamera)) _typecamera)
      (if (Utilities|Enum|Equal(Enum) _typecamera "NewEnumerator0")
        (Variables|/Game/Blueprints/Player/Camera/BP_CameraRail.BP_CameraRail_C|SetmodeTypeCamera _refcamera "NewEnumerator0")
        (bind _output_get (Variables|Default|SetActualCam (Variables|Default|GetNormalCam)))
        (Transformation|SetRelativeRotation (Variables|/Script/Engine.Actor|GetRootComponent (Variables|Default|GetRefCamera)) (Math|Conversions|RotationFromXVector _output_get) false false)
        ;[1 1 1] Position YZ from Camera only affects in the Spline position
        (Transformation|SetRelativeLocation _rootcomponent (- _returnvalue "0,400.000000,-400.000000") false false)
        (elif (Utilities|Enum|Equal(Enum) _typecamera "NewEnumerator1")
          (Variables|/Game/Blueprints/Player/Camera/BP_CameraRail.BP_CameraRail_C|SetmodeTypeCamera _refcamera "NewEnumerator1")
          (bind _output_get_2 (Variables|Default|SetActualCam (Variables|Default|GetSideScrollCam)))
          (Transformation|SetRelativeRotation (Variables|/Script/Engine.Actor|GetRootComponent (Variables|Default|GetRefCamera)) (Math|Conversions|RotationFromXVector _output_get_2) false false)
          (Transformation|SetRelativeLocation _rootcomponent (- _returnvalue "0,-400.000000,400.000000") false false)
          (else
            (Variables|/Game/Blueprints/Player/Camera/BP_CameraRail.BP_CameraRail_C|SetmodeTypeCamera _refcamera "NewEnumerator2")
            (bind _output_get_3 (Variables|Default|SetActualCam (Variables|Default|GetCombatEnemyCam)))
            (Transformation|SetRelativeRotation (Variables|/Script/Engine.Actor|GetRootComponent (Variables|Default|GetRefCamera)) (Math|Conversions|RotationFromXVector _output_get_3) false false)))))))

(fn ConstructionScript)