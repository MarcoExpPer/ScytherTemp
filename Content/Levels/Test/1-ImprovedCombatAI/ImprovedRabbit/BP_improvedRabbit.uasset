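; Improved rabbit Blueprint from a combat AI test level that switches between light and dark modes.
; Turn-dark and turn-light events, as well as construction, swap the mesh material and make the hitbox block Visibility traces only in dark mode.
; A turning-dark event drives a timeline, offset by the time to turn, that animates a material scalar to preview the change to dark.
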(event Custom|isLightMdoeChanged
  (CallFunction|LightModeChanged))

(event Custom|turningDarkEvent_Event_0
  (params (timeToTurn :type Float%20%28single-precision%29))
  (Utilities|FlowControl|Sequence
    (:then_0
      (bind _newtrack_0 (Timeline|Timeline_0 PlayFromStart)
        (:Update
          ;[1 1 1] VFX_TurningDark
          (Rendering|Material|SetScalarParameterValueonMaterials (Variables|Default|GetrabbitMesh) "AlphaChangeToDark" _newtrack_0))))
    (:then_1
      (Timeline|Timeline_0 SetNewTime))))

(event EventBeginPlay
  (|CallParentFunction)
  (EventDispatchers|AssignTurnDarkEvent (delegate Custom|isLightMdoeChanged))
  (EventDispatchers|AssignTurnLightEvent (delegate Custom|isLightMdoeChanged))
  (EventDispatchers|AssignTurningDarkEvent (delegate Custom|turningDarkEvent_Event_0)))

(fn ConstructionScript
  (CallFunction|LightModeChanged))

(fn LightModeChanged
  (Collision|SetCollisionResponsetoChannel (Variables|Default|GetrabbitHitbox) "ECC_Visibility" (select (Variables|Default|GetisLightMode) "ECR_Ignore" "ECR_Block"))
  (Rendering|Material|SetMaterial (Variables|Default|GetrabbitMesh) 0 (select (Variables|Default|GetisLightMode) (Variables|Default|GetLightMaterial) (Variables|Default|GetDarkMaterial))))